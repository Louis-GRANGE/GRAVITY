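; Rifle weapon Blueprint variant for the gravity-changing player character, built on a parent weapon class with modules.
; On BeginPlay it runs the parent setup, then removes and destroys the inherited laser module component.
; CanUse is overridden to follow the first-person character's CanChangeGravity flag, so the rifle is usable only when that character can change gravity.
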(event EventBeginPlay
  (bind _bpac_weaponmodule_laser (Variables|Default|GetBPAC_WeaponModule_Laser))
  (|CallParentFunction)
  (Utilities|Array|RemoveItem (Variables|Default|GetModules) _bpac_weaponmodule_laser)
  (Components|DestroyComponent _bpac_weaponmodule_laser))

(event Collision|EventActorBeginOverlap
  (params (OtherActor :type Actor%20Object%20Reference)))

(event EventTick
  (params (DeltaSeconds :type Float%20%28single-precision%29)))

(fn ConstructionScript
  (|CallParentFunction))

(fn CanUse
  (return (Variables|/Game/05_BP/Player/BP_GravityPlayerCharacter.BP_GravityPlayerCharacter_C|GetCanChangeGravity (Variables|Default|GetFirstPersonCharacterReference))))