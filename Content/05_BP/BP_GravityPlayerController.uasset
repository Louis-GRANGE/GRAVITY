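; Player controller for the gravity first-person character that tracks which interactable actor the player looks at.
; BeginPlay caches the character, and Tick runs a debug-drawn Visibility line trace from its camera out to InteractionRange.
; Hits implementing BPI_Interactable swap CurrentInteractable with stop/start-looking messages, but only when a valid one is already stored.
; Non-interactable hits clear the reference without a stop message, and trace misses leave it unchanged.
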(event EventBeginPlay
  (bind _asbp_gravity_first_person_character_1 (Utilities|Casting|CastToBP_gravityFirstPersonCharacter1 (Game|GetPlayerCharacter 0)))
  (Variables|Default|SetGravityCharacter _asbp_gravity_first_person_character_1))

(event EventTick
  (params (DeltaSeconds :type Float%20%28single-precision%29))
  (bind _gravitycharacter (Variables|Default|GetGravityCharacter))
  (bind _firstpersoncamera (Variables|/Game/FirstPerson/Blueprints/BP_gravityFirstPersonCharacter1.BP_gravityFirstPersonCharacter1_C|GetFirstPersonCamera _gravitycharacter))
  (bind _returnvalue (Transformation|GetWorldLocation _firstpersoncamera))
  (bind (_outhit _returnvalue_2) (Collision|LineTraceByChannel _returnvalue (+ _returnvalue (* (Math|Vector|GetForwardVector _firstpersoncamera) (Variables|Default|GetInteractionRange))) "TraceTypeQuery1" false 0 "ForOneFrame"))
  (if _returnvalue_2
    (if (Utilities|DoesObjectImplementInterface (.HitActor (Collision|BreakHitResult _outhit)) "/Game/Switches/BPI_Interactable.BPI_Interactable_C")
      (if (not (== (Variables|Default|GetCurrentInteractable) (.HitActor (Collision|BreakHitResult _outhit))))
        (Utilities|IsValid (Variables|Default|GetCurrentInteractable)
          (:Is%20Valid
            (Class|BPIInteractable|OnStopLooking(Message) (Variables|Default|GetCurrentInteractable))
            (bind _output_get (Variables|Default|SetCurrentInteractable (.HitActor (Collision|BreakHitResult _outhit))))
            (Class|BPIInteractable|OnStartLooking(Message) _output_get))))
      (else
        (Variables|Default|SetCurrentInteractable 0)))))

(fn ConstructionScript)