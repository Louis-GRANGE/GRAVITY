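; BP_CableGenerator is a placeable object that strings cables along an editable spline.
; Its construction script clears the Cables array, then adds a cable component for each pair of neighboring spline points, storing each in that array.
; Each cable's length is a tenth of the distance between its two points.
; GetGravityData returns zero direction and scale, and the event graph is empty.
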(event EventBeginPlay)

(event Collision|EventActorBeginOverlap
  (params (OtherActor :type Actor%20Object%20Reference)))

(event EventTick
  (params (DeltaSeconds :type Float%20%28single-precision%29)))

(fn ConstructionScript
  (bind _spline (Variables|Default|GetSpline))
  (Utilities|Array|Clear (Variables|Default|GetCables))
  (for _index (range 0 (- (Spline|GetNumberOfSplinePoints (Variables|Default|GetSpline)) 2))
    (bind _returnvalue (AddComponent|AddCableComponent false (Math|Transform|MakeTransform (.Location (Spline|GetLocationandTangentatSplinePoint _spline _index "Local")) "0, 0, 0" "1.000000,1.000000,1.000000")))
    (Variables|/Script/CableComponent.CableComponent|SetEndLocation _returnvalue (.Location (Spline|GetLocationandTangentatSplinePoint _spline (+ _index 1) "Local")))
    (Variables|/Script/CableComponent.CableComponent|SetCableLength _returnvalue (/ (Math|Vector|Distance(Vector) (.Location (Spline|GetLocationandTangentatSplinePoint _spline _index "Local")) (.Location (Spline|GetLocationandTangentatSplinePoint _spline (+ _index 1) "Local"))) 1e+01))
    (Utilities|Array|Add (Variables|Default|GetCables) _returnvalue)))

(fn GetGravityData
  (return "0, 0, 0" 0.0))