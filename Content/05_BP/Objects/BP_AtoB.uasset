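; BP_AtoB is an actor that moves its Cube component between the transforms of its A and B components.
; On BeginPlay it sets the Travel timeline's play rate to the inverse of LoopDuration and plays it from the start.
; Each timeline update sets the cube's world transform to a lerp of A and B, with sweep and teleport off.
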(event EventBeginPlay
  (Components|Timeline|SetPlayRate (Variables|Default|GetTravel) (/ 1.0 (Variables|Default|GetLoopDuration)))
  (bind _newtrack_0 (Timeline|Travel PlayFromStart)
    (:Update
      (Transformation|SetWorldTransform (Variables|Default|GetCube) (Math|Transform|Lerp(Transform) (Transformation|GetWorldTransform (Variables|Default|GetA)) (Transformation|GetWorldTransform (Variables|Default|GetB)) _newtrack_0) false false))))

(event Collision|EventActorBeginOverlap
  (params (OtherActor :type Actor%20Object%20Reference)))

(event EventTick
  (params (DeltaSeconds :type Float%20%28single-precision%29)))

(fn ConstructionScript)