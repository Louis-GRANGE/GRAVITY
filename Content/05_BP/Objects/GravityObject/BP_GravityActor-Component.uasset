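; BP_GravityActor-Component is a physics object whose gravity can be changed through a gravity component.
; UpdateGravity forwards incoming gravity data to BPGravityComponent, while GetGravityData returns a zero direction and scale.
; It stores its spawn transform on BeginPlay, and OnActorGoOutside zeroes the mesh's linear and angular velocity and restores that transform.
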(event EventBeginPlay
  (Variables|Default|SetInitTransform (Transformation|GetActorTransform)))

(event EventTick
  (params (DeltaSeconds :type Float%20%28single-precision%29)))

(event EventUpdateGravity
  (params (Data :type S%20Gravity%20Data%20Structure))
  (Default|UpdateGravity (Variables|Default|GetBP_GravityComponent) Data))

(event Collision|EventActorBeginOverlap
  (params (OtherActor :type Actor%20Object%20Reference)))

(event EventOnActorGoOutside
  (bind _staticmesh (Variables|Default|GetStaticMesh))
  (Physics|SetPhysicsLinearVelocity _staticmesh "0, 0, 0" false "None")
  (Class|PrimitiveComponent|SetPhysicsAngularVelocityinDegrees _staticmesh "0, 0, 0" false "None")
  (Transformation|SetActorTransform (Variables|Default|GetInitTransform)))

(fn ConstructionScript)

(fn GetGravityData
  (return "0, 0, 0" 0.0))