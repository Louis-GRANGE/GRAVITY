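; Overlap-triggered activator that presses a portal button and, after TimeToActivate, sends activate messages to its linked actors.
; During the delay, a looping timer slides ActivatingSphere along the spline with fireball Niagara effects active.
; Ending overlap in "Keep on" mode cancels this, resets the sphere and button, and deactivates linked actors.
; The construction script builds cable components between consecutive spline points.
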(event OnComponentBeginOverlap(Sphere)
  (params (OverlappedComponent :type Primitive%20Component%20Object%20Reference) (OtherActor :type Actor%20Object%20Reference) (OtherComp :type Primitive%20Component%20Object%20Reference) (OtherBodyIndex :type Integer) (bFromSweep :type Boolean) (SweepResult :type Hit%20Result%20Structure%20%28by%20ref%29))
  (Variables|Default|SetIsActivated true)
  (Class|BPIActivator|Activate(Message) self)
  (bind _asabp_button (Utilities|Casting|CastToABP_Button (Components|SkeletalMesh|GetAnimInstance (Variables|Default|GetPortalButton))))
  (Variables|/Game/03_3D/Portal-Button/ABP_Button.ABP_Button_C|SetbIsPress _asabp_button true)
  (Variables|Default|SetCurrentActivatingTime 0.0)
  (bind _returnvalue (Utilities|Time|SetTimerbyEvent (EventDispatchers|CreateEvent :!event Custom|OnActivating) 0.01 true))
  (Variables|Default|SetEvt_OnActivating _returnvalue)
  (Components|Activation|Activate (Variables|Default|GetNS_FireBalls) true)
  (Utilities|FlowControl|RetriggerableDelay (Variables|Default|GetTimeToActivate))
  (if (Variables|Default|GetIsActivated)
    (CallFunction|ActivateLinkedActors)))

(event OnComponentEndOverlap(Sphere)
  (params (OverlappedComponent :type Primitive%20Component%20Object%20Reference) (OtherActor :type Actor%20Object%20Reference) (OtherComp :type Primitive%20Component%20Object%20Reference) (OtherBodyIndex :type Integer))
  (switch Utilities|FlowControl|Switch|SwitchonE_PressTypeButton (Variables|Default|GetTypeActivation)
    (:NewEnumerator1
      (Variables|Default|SetIsActivated false)
      (Class|BPIActivator|Desactivate(Message) self)
      (Utilities|Time|ClearandInvalidateTimerbyHandle (Variables|Default|GetEvt_OnActivating))
      (Components|Activation|Deactivate (Variables|Default|GetNS_FireBalls))
      (Transformation|SetRelativeLocation (Variables|Default|GetActivatingSphere) "0, 0, 0" false false)
      (CallFunction|DesactivateLinkedActors)
      (bind _asabp_button (Utilities|Casting|CastToABP_Button (Components|SkeletalMesh|GetAnimInstance (Variables|Default|GetPortalButton))))
      (Variables|/Game/03_3D/Portal-Button/ABP_Button.ABP_Button_C|SetbIsPress _asabp_button false))))

(event Custom|OnActivating
  (Variables|Default|SetCurrentActivatingTime (+ (Variables|Default|GetCurrentActivatingTime) 0.01))
  (Transformation|SetWorldLocation (Variables|Default|GetActivatingSphere) (Spline|GetLocationatTime (Variables|Default|GetSpline) (/ (Variables|Default|GetCurrentActivatingTime) (Variables|Default|GetTimeToActivate)) "World" true) false false))

(event EventBeginPlay)

(event EventTick
  (params (DeltaSeconds :type Float%20%28single-precision%29)))

(event EventActivate)

(event EventDesactivate)

(fn ConstructionScript
  (CallFunction|GenerateCablebySpline (Variables|Default|GetSpline)))

(fn ActivateLinkedActors
  (for _array_element (Variables|Default|GetLinkedTo)
    (Class|BPIActivator|Activate(Message) _array_element)))

(fn DesactivateLinkedActors
  (for _array_element (Variables|Default|GetLinkedTo)
    (Class|BPIActivator|Desactivate(Message) _array_element)))

(fn GenerateCablebySpline
  (params (Target :type Spline%20Component%20Object%20Reference))
  (for _index (range 0 (- (Spline|GetNumberOfSplinePoints Target) 2))
    (bind _returnvalue (AddComponent|AddCableComponent false (Math|Transform|MakeTransform (.Location (Spline|GetLocationandTangentatSplinePoint Target _index "Local")) "0, 0, 0" "1.000000,1.000000,1.000000")))
    (Variables|/Script/CableComponent.CableComponent|SetEndLocation _returnvalue (.Location (Spline|GetLocationandTangentatSplinePoint Target (+ _index 1) "Local")))
    (Variables|/Script/CableComponent.CableComponent|SetCableLength _returnvalue (/ (Math|Vector|Distance(Vector) (.Location (Spline|GetLocationandTangentatSplinePoint Target _index "Local")) (.Location (Spline|GetLocationandTangentatSplinePoint Target (+ _index 1) "Local"))) 1e+02))))

(fn IsActivate
  (return (Variables|Default|GetIsActivated)))