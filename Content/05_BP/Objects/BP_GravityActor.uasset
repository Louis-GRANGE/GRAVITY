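; BP_GravityActor is an actor whose static mesh is pushed by a custom, changeable gravity.
; OnGravityChange stores direction times scale times mesh mass as CurrentGravity, which Tick applies as a force with AccelChange enabled, so mass does not divide out.
; BeginPlay casts the game mode to BP_FirstPersonGameMode, but the node binding to its gravity-change dispatcher is disconnected, so this file never subscribes to changes.
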(event Custom|OnGravityChange
  (params (Direction :type Vector) (Scale :type Float%20%28double-precision%29))
  (Variables|Default|SetCurrentGravity (* Direction (* Scale (Physics|GetMass (Variables|Default|GetStaticMesh))))))

(event EventBeginPlay
  (bind _asbp_first_person_game_mode (Utilities|Casting|CastToBP_FirstPersonGameMode (Game|GetGameMode))))

(event EventTick
  (params (DeltaSeconds :type Float%20%28single-precision%29))
  (Physics|AddForce (Variables|Default|GetStaticMesh) (Variables|Default|GetCurrentGravity) "None" true))

(fn ConstructionScript)