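; BP_Door is a sliding double door that opens on Activate and closes on Desactivate.
; A single timeline drives its alpha into lerps that slide Cube and Cube1 apart along their relative X axis, and reversing it brings them back together.
; IsActivate always returns false, so it does not report the door's state.
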(event EventBeginPlay)

(event Collision|EventActorBeginOverlap
  (params (OtherActor :type Actor%20Object%20Reference)))

(event EventTick
  (params (DeltaSeconds :type Float%20%28single-precision%29)))

(event EventActivate
  (bind _cube1 (Variables|Default|GetCube1))
  (bind _cube (Variables|Default|GetCube))
  (bind _relativelocation (Variables|/Script/Engine.SceneComponent|GetRelativeLocation _cube1))
  (bind _relativelocation_2 (Variables|/Script/Engine.SceneComponent|GetRelativeLocation _cube))
  (bind _alpha (Timeline|Timeline_0 Play)
    (:Update
      (Transformation|SetRelativeLocation _cube (Math|Vector|MakeVector (Math|Float|Lerp -5e+01 -1.4e+02 _alpha) (.y _relativelocation_2) (.z _relativelocation_2)) false false)
      (Transformation|SetRelativeLocation _cube1 (Math|Vector|MakeVector (Math|Float|Lerp 5e+01 1.4e+02 _alpha) (.y _relativelocation) (.z _relativelocation)) false false))))

(event EventDesactivate
  (bind _cube1 (Variables|Default|GetCube1))
  (bind _cube (Variables|Default|GetCube))
  (bind _relativelocation (Variables|/Script/Engine.SceneComponent|GetRelativeLocation _cube1))
  (bind _relativelocation_2 (Variables|/Script/Engine.SceneComponent|GetRelativeLocation _cube))
  (bind _alpha (Timeline|Timeline_0 Reverse)
    (:Update
      (Transformation|SetRelativeLocation _cube (Math|Vector|MakeVector (Math|Float|Lerp -5e+01 -1.4e+02 _alpha) (.y _relativelocation_2) (.z _relativelocation_2)) false false)
      (Transformation|SetRelativeLocation _cube1 (Math|Vector|MakeVector (Math|Float|Lerp 5e+01 1.4e+02 _alpha) (.y _relativelocation) (.z _relativelocation)) false false))))

(fn ConstructionScript)

(fn IsActivate
  (return false))