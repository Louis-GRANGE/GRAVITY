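; Activator button that triggers its linked actors after a loading phase and releases them when deactivated.
; Activate starts the loader and sets IsPress on the PortalButton's ABP_Button anim instance to show the press.
; FinishActivated activates the linked actors.
; Desactivate deactivates them, resets and stops the loader, and clears the press flag.
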(event EventBeginPlay
  (|CallParentFunction) ; This node is disabled and will not be called.\nDrag off pins to build functionality.
)

(event Collision|EventActorBeginOverlap
  (params (OtherActor :type Actor%20Object%20Reference)))

(event EventTick
  (params (DeltaSeconds :type Float%20%28single-precision%29))
  (|CallParentFunction DeltaSeconds) ; This node is disabled and will not be called.\nDrag off pins to build functionality.
)

(event EventActivate
  (CallFunction|Loader-Start)
  (bind _asabp_button (Utilities|Casting|CastToABP_Button (Components|SkeletalMesh|GetAnimInstance (Variables|Default|GetPortalButton))))
  (Variables|/Game/03_3D/Portal-Button/ABP_Button.ABP_Button_C|SetbIsPress _asabp_button true))

(event EventDesactivate
  (CallFunction|DesactivateLinkedActors)
  (CallFunction|Loader-Restartat 0.0)
  (CallFunction|Loader-Stop)
  (bind _asabp_button (Utilities|Casting|CastToABP_Button (Components|SkeletalMesh|GetAnimInstance (Variables|Default|GetPortalButton))))
  (Variables|/Game/03_3D/Portal-Button/ABP_Button.ABP_Button_C|SetbIsPress _asabp_button false))

(event EventFinishActivated
  (CallFunction|ActivateLinkedActors))

(fn ConstructionScript
  (|CallParentFunction))