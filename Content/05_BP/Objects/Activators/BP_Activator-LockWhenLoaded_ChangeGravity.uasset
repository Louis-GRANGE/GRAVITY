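; Activator variant, named as a lock-when-loaded type, that changes gravity while activated and restores it when deactivated.
; On BeginPlay it binds to the finish-activate and deactivated dispatchers.
; Activation caches the current world gravity direction, then applies the configured Direction through the gravity system using PortalButton's location; deactivation reapplies the cached direction.
; The construction script rotates GravityDir to preview the configured Direction.
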(event Custom|Evt_OnActivated
  (bind _returnvalue (CallFunction|GetGSGravity))
  (Variables|Default|SetBeforeActivateDirection (Variables|/Game/05_BP/GS_Gravity.GS_Gravity_C|GetWorldDirGravity _returnvalue))
  (Default|UpdateGravityto _returnvalue "NewEnumerator3" (Variables|Default|GetDirection) -9.8 (Transformation|GetWorldLocation (Variables|Default|GetPortalButton))))

(event Custom|Evt_OnDeactivated
  (Default|UpdateGravityto (CallFunction|GetGSGravity) "NewEnumerator3" (Variables|Default|GetBeforeActivateDirection) -9.8 (Transformation|GetWorldLocation (Variables|Default|GetPortalButton))))

(event EventBeginPlay
  (|CallParentFunction)
  (EventDispatchers|BindEventto+OnFinishActivate (EventDispatchers|CreateEvent :!event Custom|Evt_OnActivated))
  (EventDispatchers|BindEventto+OnDeactivated (EventDispatchers|CreateEvent :!event Custom|Evt_OnDeactivated)))

(event Collision|EventActorBeginOverlap
  (params (OtherActor :type Actor%20Object%20Reference))
  (|CallParentFunction OtherActor) ; This node is disabled and will not be called.\nDrag off pins to build functionality.
)

(event EventTick
  (params (DeltaSeconds :type Float%20%28single-precision%29))
  (|CallParentFunction DeltaSeconds) ; This node is disabled and will not be called.\nDrag off pins to build functionality.
)

(fn ConstructionScript
  (|CallParentFunction)
  (Transformation|SetWorldRotation (Variables|Default|GetGravityDir) (Math|Conversions|RotationFromXVector (Variables|Default|GetDirection)) false false))