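; Timed-lock pressure plaque activator, a child Blueprint that changes gravity when activated.
; BeginPlay binds an event to the OnFinishActivate dispatcher after the parent's setup.
; Evt_OnActivated pushes an entry onto the gravity system's stack with the configured Direction, LockDuration, GravityDir's location and itself as sender.
; The construction script rotates the GravityDir component to show Direction.
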(event Custom|Evt_OnActivated
  (Default|AddGravityStack (CallFunction|GetGSGravity) (Utilities|Struct|MakeS_GravityData (Utilities|Array|MakeArray "NewEnumerator3") (Variables|Default|GetDirection) -9.8 (Transformation|GetWorldLocation (Variables|Default|GetGravityDir)) (Variables|Default|GetLockDuration) self)))

(event EventBeginPlay
  (|CallParentFunction)
  (EventDispatchers|BindEventto+OnFinishActivate (EventDispatchers|CreateEvent :!event Custom|Evt_OnActivated)))

(event Collision|EventActorBeginOverlap
  (params (OtherActor :type Actor%20Object%20Reference))
  (|CallParentFunction OtherActor) ; This node is disabled and will not be called.\nDrag off pins to build functionality.
)

(event EventTick
  (params (DeltaSeconds :type Float%20%28single-precision%29))
  (|CallParentFunction DeltaSeconds) ; This node is disabled and will not be called.\nDrag off pins to build functionality.
)

(fn ConstructionScript
  (|CallParentFunction)
  (Transformation|SetWorldRotation (Variables|Default|GetGravityDir) (Math|Conversions|RotationFromXVector (Variables|Default|GetDirection)) false false))