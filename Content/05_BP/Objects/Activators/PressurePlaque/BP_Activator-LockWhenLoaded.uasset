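; Activator button that charges while something overlaps its sphere and is meant to lock once loading finishes.
; Activation starts the Loader and sets the button AnimBP's pressed state, while Loading feeds progress into the locker plane's IsUnlock material parameter.
; FinishActivated activates linked actors.
; Leaving the sphere before LoadFinish sends a deactivate message; Deactivate turns off linked actors, resets the Loader and releases the button.
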(event OnComponentEndOverlap(Sphere)
  (params (OverlappedComponent :type Primitive%20Component%20Object%20Reference) (OtherActor :type Actor%20Object%20Reference) (OtherComp :type Primitive%20Component%20Object%20Reference) (OtherBodyIndex :type Integer))
  (Variables|Default|SetIsActivated false)
  (if (not (Variables|Default|GetLoadFinish))
    (Class|BPIActivator|Deactivate(Message) self)))

(event OnComponentBeginOverlap(Sphere)
  (params (OverlappedComponent :type Primitive%20Component%20Object%20Reference) (OtherActor :type Actor%20Object%20Reference) (OtherComp :type Primitive%20Component%20Object%20Reference) (OtherBodyIndex :type Integer) (bFromSweep :type Boolean) (SweepResult :type Hit%20Result%20Structure%20%28by%20ref%29))
  (Variables|Default|SetIsActivated true)
  (Class|BPIActivator|Activate(Message) self))

(event EventBeginPlay
  (|CallParentFunction) ; This node is disabled and will not be called.\nDrag off pins to build functionality.
)

(event Collision|EventActorBeginOverlap
  (params (OtherActor :type Actor%20Object%20Reference)))

(event EventTick
  (params (DeltaSeconds :type Float%20%28single-precision%29))
  (|CallParentFunction DeltaSeconds) ; This node is disabled and will not be called.\nDrag off pins to build functionality.
)

(event EventActivate
  (if (not (Variables|Default|GetLoadFinish))
    (CallFunction|Loader-Start)
    (bind _asabp_button (Utilities|Casting|CastToABP_Button (Components|SkeletalMesh|GetAnimInstance (Variables|Default|GetPortalButton))))
    (Variables|/Game/03_3D/Portal-Button/ABP_Button.ABP_Button_C|SetbIsPress _asabp_button true)))

(event EventDeactivate
  (CallFunction|DesactivateLinkedActors)
  (CallFunction|Loader-Restartat 0.0)
  (CallFunction|Loader-Stop)
  (bind _asabp_button (Utilities|Casting|CastToABP_Button (Components|SkeletalMesh|GetAnimInstance (Variables|Default|GetPortalButton))))
  (Variables|/Game/03_3D/Portal-Button/ABP_Button.ABP_Button_C|SetbIsPress _asabp_button false))

(event EventFinishActivated
  (CallFunction|ActivateLinkedActors))

(event EventLoading
  (params (Time :type Float%20%28double-precision%29))
  (Rendering|Material|SetScalarParameterValueonMaterials (Variables|Default|GetLocker-Plane) "IsUnlock" Time))

(fn ConstructionScript
  (|CallParentFunction))