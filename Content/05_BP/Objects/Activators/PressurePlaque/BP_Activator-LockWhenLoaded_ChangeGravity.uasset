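; Pressure-plaque activator, child of a lock-when-loaded activator, that changes world gravity to its configured Direction.
; When activation finishes, it saves the current gravity direction and pushes a gravity stack entry at the PortalButton location.
; If reactivation is allowed, it listens for gravity changes and unlocks and deactivates when another instance applies one with duration -1.
; The construction script orients GravityDir along Direction.
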(event Custom|Evt_OnGravityChange
  (params (Data :type S%20Gravity%20Data%20Structure))
  (bind (_applyto _direction _scale _location _duration _sender) (Utilities|Struct|BreakS_GravityData Data))
  (Utilities|Casting|CastToBP_Activator-LockWhenLoaded_ChangeGravity _sender)
  (if (!= _sender self)
    (if (== _duration -1.0)
      (Variables|Default|SetLoadFinish false)
      (CallFunction|Deactivate))))

(event Custom|Evt_OnActivated
  (bind _returnvalue (CallFunction|GetGSGravity))
  (Variables|Default|SetBeforeActivateDirection (Variables|/Game/05_BP/GS_Gravity.GS_Gravity_C|GetWorldDirGravity _returnvalue))
  (Default|AddGravityStack _returnvalue (Utilities|Struct|MakeS_GravityData (Utilities|Array|MakeArray "NewEnumerator3") (Variables|Default|GetDirection) -9.8 (Transformation|GetWorldLocation (Variables|Default|GetPortalButton)) -1.0 self)))

(event EventBeginPlay
  (|CallParentFunction)
  (EventDispatchers|BindEventto+OnFinishActivate (EventDispatchers|CreateEvent :!event Custom|Evt_OnActivated))
  (if (Variables|Default|GetCanBeReactivatedAfterChangeWorldGravity)
    (EventDispatchers|BindEventtoOnGravityChange (CallFunction|GetGSGravity) (EventDispatchers|CreateEvent :!event Custom|Evt_OnGravityChange))))

(event Collision|EventActorBeginOverlap
  (params (OtherActor :type Actor%20Object%20Reference))
  (|CallParentFunction OtherActor) ; This node is disabled and will not be called.\nDrag off pins to build functionality.
)

(event EventTick
  (params (DeltaSeconds :type Float%20%28single-precision%29))
  (|CallParentFunction DeltaSeconds) ; This node is disabled and will not be called.\nDrag off pins to build functionality.
)

(fn ConstructionScript
  (|CallParentFunction)
  (Transformation|SetWorldRotation (Variables|Default|GetGravityDir) (Math|Conversions|RotationFromXVector (Variables|Default|GetDirection)) false false))