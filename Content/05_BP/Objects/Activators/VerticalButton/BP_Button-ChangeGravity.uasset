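; Button activator that changes gravity by pushing an entry onto the gravity stack fetched through GetGSGravity.
; Finishing activation adds the entry with the button's Direction, base mesh location and ActivateDuration.
; With a duration of -1, it tracks the stack index to replace the entry on reactivation and remove it on deactivation.
; The construction script rotates GravityDir to preview the direction.
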(event Custom|Evt_OnActivated
  (if (== (Variables|Default|GetActivateDuration) -1.0)
    (if (!= (Variables|Default|GetIndexGravity) -1)
      (Default|RemoveGravityStack (CallFunction|GetGSGravity) (Variables|Default|GetIndexGravity))))
  (bind _index (Default|AddGravityStack (CallFunction|GetGSGravity) (Utilities|Struct|MakeS_GravityData (Utilities|Array|MakeArray "NewEnumerator3") (Variables|Default|GetDirection) -9.8 (Transformation|GetWorldLocation (Variables|Default|GetSM_Button-Base)) (Variables|Default|GetActivateDuration) self)))
  (Variables|Default|SetIndexGravity _index))

(event Custom|Evt_OnDeactivated
  (if (== (Variables|Default|GetActivateDuration) -1.0)
    (Default|RemoveGravityStack (CallFunction|GetGSGravity) (Variables|Default|GetIndexGravity))
    (Variables|Default|SetIndexGravity -1)))

(event EventBeginPlay
  (|CallParentFunction)
  (EventDispatchers|BindEventto+OnFinishActivate (EventDispatchers|CreateEvent :!event Custom|Evt_OnActivated))
  (EventDispatchers|BindEventto+OnDeactivated (EventDispatchers|CreateEvent :!event Custom|Evt_OnDeactivated)))

(event Collision|EventActorBeginOverlap
  (params (OtherActor :type Actor%20Object%20Reference)))

(event EventTick
  (params (DeltaSeconds :type Float%20%28single-precision%29))
  (|CallParentFunction DeltaSeconds) ; This node is disabled and will not be called.\nDrag off pins to build functionality.
)

(fn ConstructionScript
  (|CallParentFunction)
  (Transformation|SetWorldRotation (Variables|Default|GetGravityDir) (Math|Conversions|RotationFromXVector (Variables|Default|GetDirection)) false false))