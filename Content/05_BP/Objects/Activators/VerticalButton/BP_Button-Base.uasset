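; Base pressable button that runs a timed activation loader and can notify linked actors on activation and deactivation.
; The construction script strings cable components between spline points.
; A press timeline sinks the button and starts the loader, which moves a sphere along the spline, toggles fireball effects and fills each cable's material "%" parameter.
; After a delay the button pops up, subject to press-limit settings, deactivating linked actors and resetting the loader.
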(event Custom|Loader-Start
  (bind _spline (Variables|Default|GetSpline))
  (bind _returnvalue (Spline|GetSplineLength _spline))
  ;[0.1719 0 0] Loader
  (Variables|Default|SetCurrentIndexCable 0)
  (Rendering|SetVisibility (Variables|Default|GetActivatingSphere) true false)
  (Components|Activation|Activate (Variables|Default|GetNS_FireBalls) true)
  (Components|Timeline|SetPlayRate (Variables|Default|GetTL_Loader) (/ 1.0 (Variables|Default|GetTimeToActivate)))
  (Variables|Default|SetLoadFinish false)
  (bind (_direction _alpha) (Timeline|TL_Loader PlayFromStart)
    (:Update
      (CallFunction|Loading _alpha)
      (Transformation|SetWorldLocation (Variables|Default|GetActivatingSphere) (Spline|GetLocationatTime _spline _alpha "World" true) false false)
      (if (>= _alpha (/ (Spline|GetDistanceAlongSplineatSplinePoint _spline (Variables|Default|GetCurrentIndexCable)) _returnvalue))
        (if (> (Variables|Default|GetCurrentIndexCable) 0)
          (Rendering|Material|SetScalarParameterValueonMaterials (Utilities|Array|Get(acopy) (Variables|Default|GetCables) (- (Variables|Default|GetCurrentIndexCable) 1)) "%" 1.0))
        (Math|Integer|IncrementInt (Variables|Default|GetCurrentIndexCable))
        (elif (> (Variables|Default|GetCurrentIndexCable) 0)
          (Rendering|Material|SetScalarParameterValueonMaterials (Utilities|Array|Get(acopy) (Variables|Default|GetCables) (- (Variables|Default|GetCurrentIndexCable) 1)) "%" (Math|Float|MapRangeClamped _alpha (/ (Spline|GetDistanceAlongSplineatSplinePoint _spline (- (Variables|Default|GetCurrentIndexCable) 1)) _returnvalue) (/ (Spline|GetDistanceAlongSplineatSplinePoint _spline (Variables|Default|GetCurrentIndexCable)) _returnvalue) 0.0 0.9)))))
    (:Finished
      (switch Utilities|FlowControl|Switch|SwitchonETimelineDirection _direction
        (:Forward
          (Variables|Default|SetLoadFinish true)
          (Components|Activation|Deactivate (Variables|Default|GetNS_FireBalls))
          (Rendering|SetVisibility (Variables|Default|GetActivatingSphere) false false)
          (Class|BPIActivator|FinishActivated(Message) self))))))

(event Custom|Loader-RestartAt
  (params (Time :type Float%20%28double-precision%29))
  (bind _spline (Variables|Default|GetSpline))
  (bind _returnvalue (Spline|GetSplineLength _spline))
  ;[0.1719 0 0] Loader
  (Components|Activation|Deactivate (Variables|Default|GetNS_FireBalls))
  (CallFunction|ResetPercentMaterialCable)
  (Rendering|SetVisibility (Variables|Default|GetActivatingSphere) false false)
  (Variables|Default|SetCurrentIndexCable 0)
  (Variables|Default|SetLoadFinish false)
  (bind (_direction _alpha) (Timeline|TL_Loader SetNewTime)
    (:Update
      (CallFunction|Loading _alpha)
      (Transformation|SetWorldLocation (Variables|Default|GetActivatingSphere) (Spline|GetLocationatTime _spline _alpha "World" true) false false)
      (if (>= _alpha (/ (Spline|GetDistanceAlongSplineatSplinePoint _spline (Variables|Default|GetCurrentIndexCable)) _returnvalue))
        (if (> (Variables|Default|GetCurrentIndexCable) 0)
          (Rendering|Material|SetScalarParameterValueonMaterials (Utilities|Array|Get(acopy) (Variables|Default|GetCables) (- (Variables|Default|GetCurrentIndexCable) 1)) "%" 1.0))
        (Math|Integer|IncrementInt (Variables|Default|GetCurrentIndexCable))
        (elif (> (Variables|Default|GetCurrentIndexCable) 0)
          (Rendering|Material|SetScalarParameterValueonMaterials (Utilities|Array|Get(acopy) (Variables|Default|GetCables) (- (Variables|Default|GetCurrentIndexCable) 1)) "%" (Math|Float|MapRangeClamped _alpha (/ (Spline|GetDistanceAlongSplineatSplinePoint _spline (- (Variables|Default|GetCurrentIndexCable) 1)) _returnvalue) (/ (Spline|GetDistanceAlongSplineatSplinePoint _spline (Variables|Default|GetCurrentIndexCable)) _returnvalue) 0.0 0.9)))))
    (:Finished
      (switch Utilities|FlowControl|Switch|SwitchonETimelineDirection _direction
        (:Forward
          (Variables|Default|SetLoadFinish true)
          (Components|Activation|Deactivate (Variables|Default|GetNS_FireBalls))
          (Rendering|SetVisibility (Variables|Default|GetActivatingSphere) false false)
          (Class|BPIActivator|FinishActivated(Message) self))))))

(event Custom|Loader-Stop
  (bind _spline (Variables|Default|GetSpline))
  (bind _currentindexcable (Variables|Default|GetCurrentIndexCable))
  (bind _currentindexcable_2 (Variables|Default|GetCurrentIndexCable))
  (bind _currentindexcable_3 (Variables|Default|GetCurrentIndexCable))
  (bind _returnvalue (Spline|GetDistanceAlongSplineatSplinePoint _spline _currentindexcable_2))
  (bind _returnvalue_2 (Spline|GetSplineLength _spline))
  (bind _returnvalue_3 (/ _returnvalue _returnvalue_2))
  ;[0.1719 0 0] Loader
  (Components|Activation|Deactivate (Variables|Default|GetNS_FireBalls))
  (Rendering|SetVisibility (Variables|Default|GetActivatingSphere) false false)
  (Variables|Default|SetLoadFinish false)
  (bind (_direction _alpha) (Timeline|TL_Loader Stop)
    (:Update
      (CallFunction|Loading _alpha)
      (Transformation|SetWorldLocation (Variables|Default|GetActivatingSphere) (Spline|GetLocationatTime _spline _alpha "World" true) false false)
      (if (>= _alpha _returnvalue_3)
        (if (> _currentindexcable_3 0)
          (Rendering|Material|SetScalarParameterValueonMaterials (Utilities|Array|Get(acopy) (Variables|Default|GetCables) (- _currentindexcable_3 1)) "%" 1.0))
        (Math|Integer|IncrementInt (Variables|Default|GetCurrentIndexCable))
        (elif (> _currentindexcable 0)
          (Rendering|Material|SetScalarParameterValueonMaterials (Utilities|Array|Get(acopy) (Variables|Default|GetCables) (- _currentindexcable 1)) "%" (Math|Float|MapRangeClamped _alpha (/ (Spline|GetDistanceAlongSplineatSplinePoint _spline (- _currentindexcable_2 1)) _returnvalue_2) _returnvalue_3 0.0 0.9)))))
    (:Finished
      (switch Utilities|FlowControl|Switch|SwitchonETimelineDirection _direction
        (:Forward
          (Variables|Default|SetLoadFinish true)
          (Components|Activation|Deactivate (Variables|Default|GetNS_FireBalls))
          (Rendering|SetVisibility (Variables|Default|GetActivatingSphere) false false)
          (Class|BPIActivator|FinishActivated(Message) self))))))

(event Custom|Loader-Continue
  (bind _spline (Variables|Default|GetSpline))
  (bind _currentindexcable (Variables|Default|GetCurrentIndexCable))
  (bind _currentindexcable_2 (Variables|Default|GetCurrentIndexCable))
  (bind _currentindexcable_3 (Variables|Default|GetCurrentIndexCable))
  (bind _returnvalue (Spline|GetDistanceAlongSplineatSplinePoint _spline _currentindexcable_2))
  (bind _returnvalue_2 (Spline|GetSplineLength _spline))
  (bind _returnvalue_3 (/ _returnvalue _returnvalue_2))
  ;[0.1719 0 0] Loader
  (Components|Activation|Activate (Variables|Default|GetNS_FireBalls) true)
  (Rendering|SetVisibility (Variables|Default|GetActivatingSphere) true false)
  (Variables|Default|SetLoadFinish false)
  (bind (_direction _alpha) (Timeline|TL_Loader Play)
    (:Update
      (CallFunction|Loading _alpha)
      (Transformation|SetWorldLocation (Variables|Default|GetActivatingSphere) (Spline|GetLocationatTime _spline _alpha "World" true) false false)
      (if (>= _alpha _returnvalue_3)
        (if (> _currentindexcable_3 0)
          (Rendering|Material|SetScalarParameterValueonMaterials (Utilities|Array|Get(acopy) (Variables|Default|GetCables) (- _currentindexcable_3 1)) "%" 1.0))
        (Math|Integer|IncrementInt (Variables|Default|GetCurrentIndexCable))
        (elif (> _currentindexcable 0)
          (Rendering|Material|SetScalarParameterValueonMaterials (Utilities|Array|Get(acopy) (Variables|Default|GetCables) (- _currentindexcable 1)) "%" (Math|Float|MapRangeClamped _alpha (/ (Spline|GetDistanceAlongSplineatSplinePoint _spline (- _currentindexcable_2 1)) _returnvalue_2) _returnvalue_3 0.0 0.9)))))
    (:Finished
      (switch Utilities|FlowControl|Switch|SwitchonETimelineDirection _direction
        (:Forward
          (Variables|Default|SetLoadFinish true)
          (Components|Activation|Deactivate (Variables|Default|GetNS_FireBalls))
          (Rendering|SetVisibility (Variables|Default|GetActivatingSphere) false false)
          (Class|BPIActivator|FinishActivated(Message) self))))))

(event Custom|Loader-Reverse
  (bind _spline (Variables|Default|GetSpline))
  (bind _currentindexcable (Variables|Default|GetCurrentIndexCable))
  (bind _currentindexcable_2 (Variables|Default|GetCurrentIndexCable))
  (bind _currentindexcable_3 (Variables|Default|GetCurrentIndexCable))
  (bind _returnvalue (Spline|GetDistanceAlongSplineatSplinePoint _spline _currentindexcable_2))
  (bind _returnvalue_2 (Spline|GetSplineLength _spline))
  (bind _returnvalue_3 (/ _returnvalue _returnvalue_2))
  ;[0.1719 0 0] Loader
  (Components|Activation|Activate (Variables|Default|GetNS_FireBalls) true)
  (Rendering|SetVisibility (Variables|Default|GetActivatingSphere) true false)
  (Variables|Default|SetLoadFinish false)
  (bind (_direction _alpha) (Timeline|TL_Loader Reverse)
    (:Update
      (CallFunction|Loading _alpha)
      (Transformation|SetWorldLocation (Variables|Default|GetActivatingSphere) (Spline|GetLocationatTime _spline _alpha "World" true) false false)
      (if (>= _alpha _returnvalue_3)
        (if (> _currentindexcable_3 0)
          (Rendering|Material|SetScalarParameterValueonMaterials (Utilities|Array|Get(acopy) (Variables|Default|GetCables) (- _currentindexcable_3 1)) "%" 1.0))
        (Math|Integer|IncrementInt (Variables|Default|GetCurrentIndexCable))
        (elif (> _currentindexcable 0)
          (Rendering|Material|SetScalarParameterValueonMaterials (Utilities|Array|Get(acopy) (Variables|Default|GetCables) (- _currentindexcable 1)) "%" (Math|Float|MapRangeClamped _alpha (/ (Spline|GetDistanceAlongSplineatSplinePoint _spline (- _currentindexcable_2 1)) _returnvalue_2) _returnvalue_3 0.0 0.9)))))
    (:Finished
      (switch Utilities|FlowControl|Switch|SwitchonETimelineDirection _direction
        (:Forward
          (Variables|Default|SetLoadFinish true)
          (Components|Activation|Deactivate (Variables|Default|GetNS_FireBalls))
          (Rendering|SetVisibility (Variables|Default|GetActivatingSphere) false false)
          (Class|BPIActivator|FinishActivated(Message) self))))))

(event Custom|Loading
  (params (Time :type Float%20%28double-precision%29))
  ;[0.1719 0 0] Loader
)

(event Custom|UpButton
  (bind (_direction _alpha) (Timeline|TL_Press Reverse)
    (:Update
      (Transformation|SetRelativeLocation (Variables|Default|GetRootButton-Press) (Math|Vector|Lerp(Vector) "0, 0, 0" "15.000000, 0, 0" _alpha) false false))
    (:Finished
      (switch Utilities|FlowControl|Switch|SwitchonETimelineDirection _direction
        (:Forward
          (CallFunction|Activate)
          (CallFunction|Loader-Start)
          (Utilities|FlowControl|Delay (+ (Variables|Default|GetTimeToActivate) (Variables|Default|GetActivateTime)))
          (if (Variables|Default|GetInifityPress)
            (CallFunction|UpButton :!label _label)
            (elif (< (Variables|Default|GetCurrentNbPress) (Variables|Default|GetMaxNbPress))
              (goto _label))))
        (:Backward
          (Variables|Default|SetIsButtonDown false)
          (CallFunction|Desactivate)
          (CallFunction|DesactivateLinkedActors)
          (CallFunction|Loader-Restartat 0.0)
          (CallFunction|Loader-Stop))))))

(event EventBeginPlay)

(event EventOnPress
  (params (PlayerRef :type BP%20Gravity%20Player%20Character%20Object%20Reference) (Input :type Key%20Structure :default "None"))
  (if (not (Variables|Default|GetIsButtonDown))
    (Variables|Default|SetIsButtonDown true)
    (if (Variables|Default|GetInifityPress)
      (bind (_direction _alpha) (Timeline|TL_Press Play)
        (:Update
          (Transformation|SetRelativeLocation (Variables|Default|GetRootButton-Press) (Math|Vector|Lerp(Vector) "0, 0, 0" "15.000000, 0, 0" _alpha) false false))
        (:Finished
          (switch Utilities|FlowControl|Switch|SwitchonETimelineDirection _direction
            (:Forward
              (CallFunction|Activate)
              (CallFunction|Loader-Start)
              (Utilities|FlowControl|Delay (+ (Variables|Default|GetTimeToActivate) (Variables|Default|GetActivateTime)))
              (if (Variables|Default|GetInifityPress)
                (CallFunction|UpButton :!label _label)
                (elif (< (Variables|Default|GetCurrentNbPress) (Variables|Default|GetMaxNbPress))
                  (goto _label))))
            (:Backward
              (Variables|Default|SetIsButtonDown false)
              (CallFunction|Desactivate)
              (CallFunction|DesactivateLinkedActors)
              (CallFunction|Loader-Restartat 0.0)
              (CallFunction|Loader-Stop)))))
      (else
        (bind _result (Math|Integer|IncrementInt (Variables|Default|GetCurrentNbPress))
          (:%20%20
            (if (<= _result (Variables|Default|GetMaxNbPress))
              (Timeline|TL_Press Play))))))))

(event EventTick
  (params (DeltaSeconds :type Float%20%28single-precision%29)))

(event EventDesactivate)

(fn ConstructionScript
  (CallFunction|GenerateCablebySpline (Variables|Default|GetSpline)))

(fn ActivateLinkedActors
  (for _array_element (Variables|Default|GetLinkedTo)
    (Class|BPIActivator|Activate(Message) _array_element))
  (Default|Call+OnFinishActivate))

(fn DesactivateLinkedActors
  (for _array_element (Variables|Default|GetLinkedTo)
    (Class|BPIActivator|Desactivate(Message) _array_element))
  (Default|Call+OnDeactivated))

(fn GenerateCablebySpline
  (params (Target :type Spline%20Component%20Object%20Reference))
  (bind _relativelocation (Variables|/Script/Engine.SceneComponent|GetRelativeLocation Target))
  (Utilities|Array|Clear (Variables|Default|GetCables))
  (for _index (range 0 (- (Spline|GetNumberOfSplinePoints Target) 2))
    (bind _returnvalue (AddComponent|AddCableComponent false (Math|Transform|MakeTransform (+ (.Location (Spline|GetLocationandTangentatSplinePoint Target _index "Local")) _relativelocation) "0, 0, 0" "1.000000,1.000000,1.000000")))
    (Variables|/Script/CableComponent.CableComponent|SetEndLocation _returnvalue (+ (.Location (Spline|GetLocationandTangentatSplinePoint Target (+ _index 1) "Local")) _relativelocation))
    (Variables|/Script/CableComponent.CableComponent|SetCableLength _returnvalue (/ (Math|Vector|Distance(Vector) (+ (.Location (Spline|GetLocationandTangentatSplinePoint Target _index "Local")) _relativelocation) (+ (.Location (Spline|GetLocationandTangentatSplinePoint Target (+ _index 1) "Local")) _relativelocation)) 1e+02))
    (Utilities|Array|Add (Variables|Default|GetCables) _returnvalue)))

(fn ResetPercentMaterialCable
  (for _array_element (Variables|Default|GetCables)
    (Rendering|Material|SetScalarParameterValueonMaterials _array_element "%" 0.0)))

(fn IsActivate
  (return (Variables|Default|GetIsActivated)))