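; Player controller for the gravity game that handles interaction, pausing and an F key that shows the scoreboard and finishes the run level.
; Each tick, a camera line trace caches the nearby BPI_Interactable actor and sends hover changes; Use press and release are forwarded to it.
; Unhover fires only when switching interactables; a non-interactable hit in range clears the target silently, while misses or distant hits keep it.
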(event EventBeginPlay
  (bind _asbp_gravity_player_character (Utilities|Casting|CastToBP_GravityPlayerCharacter (Game|GetPlayerCharacter 0)))
  (Variables|Default|SetGravityCharacter _asbp_gravity_player_character))

(event EventTick
  (params (DeltaSeconds :type Float%20%28single-precision%29))
  (CallFunction|Interactables))

(event Input|ActionEvents|InputActionPause
  (params (Key :type Key%20Structure :default "None"))
  (:Pressed
    (bind _asbpgm_gravity_game (Utilities|Casting|CastToBPGM_GravityGame (Game|GetGameMode)))
    (Default|SetGamePause _asbpgm_gravity_game (not (Game|IsGamePaused)))))

(event Input|ActionEvents|InputActionUse
  (params (Key :type Key%20Structure :default "None"))
  (bind _currentinteractable (Variables|Default|GetCurrentInteractable))
  (bind _gravitycharacter (Variables|Default|GetGravityCharacter))
  (:Pressed
    (Class|BPIInteractable|OnPress(Message) _currentinteractable _gravitycharacter Key))
  (:Released
    (Class|BPIInteractable|OnRelease(Message) _currentinteractable _gravitycharacter Key)))

(event Input|KeyboardEvents|F
  (params (Key :type Key%20Structure :default "None"))
  (:Pressed
    (bind _ashud_in_game (Utilities|Casting|CastToHUD_InGame (HUD|GetHUD)))
    (Default|ShowScoreboard _ashud_in_game)
    (Default|FinishRunLevel (CallFunction|GetGIGravity))))

(fn ConstructionScript)

(fn Interactables
  (bind _gravitycharacter (Variables|Default|GetGravityCharacter))
  (bind _firstpersoncamera (Variables|/Game/05_BP/Player/BP_GravityPlayerCharacter.BP_GravityPlayerCharacter_C|GetFirstPersonCamera _gravitycharacter))
  (bind _returnvalue (Transformation|GetWorldLocation _firstpersoncamera))
  (Utilities|IsValid _gravitycharacter
    (:Is%20Valid
      (bind (_outhit _returnvalue_2) (Collision|LineTraceByChannel _returnvalue (+ _returnvalue (* (Math|Vector|GetForwardVector _firstpersoncamera) 999999999999.0)) "TraceTypeQuery1" false 0 "None"))
      (bind _output_get (Variables|Default|SetHitForwardCamera _outhit))
      (if _returnvalue_2
        (if (< (.Distance (Collision|BreakHitResult _output_get)) (Variables|Default|GetInteractionRange))
          (if (Utilities|DoesObjectImplementInterface (.HitActor (Collision|BreakHitResult _output_get)) "/Game/05_BP/Switches/BPI_Interactable.BPI_Interactable_C")
            (if (not (== (Variables|Default|GetCurrentInteractable) (.HitActor (Collision|BreakHitResult _output_get))))
              (Utilities|IsValid (Variables|Default|GetCurrentInteractable)
                (:Is%20Valid
                  (Class|BPIInteractable|OnUnHover(Message) (Variables|Default|GetCurrentInteractable) (Variables|Default|GetGravityCharacter)))
                (:Is%20Not%20Valid
                  _))
              (bind _output_get_2 (Variables|Default|SetCurrentInteractable (.HitActor (Collision|BreakHitResult _output_get))))
              (Class|BPIInteractable|OnHover(Message) _output_get_2 (Variables|Default|GetGravityCharacter)))
            (else
              (Variables|Default|SetCurrentInteractable 0))))))))