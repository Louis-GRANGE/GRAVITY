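; Player controller for the level editor, providing fly-camera navigation alongside a cursor-driven editor UI.
; By default it shows the cursor and uses Game and UI input focused on the main level editor widget from the HUD.
; Holding SecondaryAction hides the cursor, switches to game-only input and enables pawn movement and mouse look relative to control rotation.
; Each toggle broadcasts the CanMove state through CallOnCanMove.
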(event EventBeginPlay
  (Variables|Default|SetbShowMouseCursor true)
  (Input|SetInputModeGameandUI self (Variables|/Game/05_BP/LevelEditor/HUD_LevelEditor.HUD_LevelEditor_C|GetWBP_MainLevelEditor (.AsHUD%20Level%20Editor (Utilities|Casting|CastToHUD_LevelEditor (HUD|GetHUD)))) "LockInFullscreen" false))

(event Input|ActionEvents|InputActionSecondaryAction
  (params (Key :type Key%20Structure :default "None"))
  (:Pressed
    (Variables|Default|SetCanMove true)
    (Variables|Default|SetbShowMouseCursor false)
    (Input|SetInputModeGameOnly self)
    (Default|Call+OnCanMove (Variables|Default|GetCanMove)))
  (:Released
    (Variables|Default|SetCanMove false)
    (Variables|Default|SetbShowMouseCursor true)
    (Input|SetInputModeGameandUI self (Variables|/Game/05_BP/LevelEditor/HUD_LevelEditor.HUD_LevelEditor_C|GetWBP_MainLevelEditor (.AsHUD%20Level%20Editor (Utilities|Casting|CastToHUD_LevelEditor (HUD|GetHUD)))) "LockInFullscreen" false)
    (Default|Call+OnCanMove (Variables|Default|GetCanMove))))

(event Input|AxisEvents|InputAxisMoveForward
  (params (AxisValue :type Float%20%28single-precision%29))
  (bind _returnvalue (Pawn|GetControlledPawn))
  ;[0.5034 1 0.92] Movements
  ;;[1 0.9233 0.156] Move Forward/Backward
  (if (Variables|Default|GetCanMove)
    (Pawn|Input|AddMovementInput _returnvalue (* AxisValue (Math|Vector|GetForwardVector (Pawn|GetControlRotation _returnvalue :!class /Script/Engine.Pawn))) (Variables|Default|GetMoveSpeed) false)))

(event Input|AxisEvents|InputAxisMoveUp/Down
  (params (AxisValue :type Float%20%28single-precision%29))
  ;[0.5034 1 0.92] Movements
  ;;[1 0.3801 0.6368] Move Up/Down
  (if (Variables|Default|GetCanMove)
    (Pawn|Input|AddMovementInput (Pawn|GetControlledPawn) (* AxisValue "0,0,1.000000") (Variables|Default|GetMoveSpeed) false)))

(event Input|AxisEvents|InputAxisLookUp/DownMouse
  (params (AxisValue :type Float%20%28single-precision%29))
  (if (Variables|Default|GetCanMove)
    (Pawn|Input|AddControllerPitchInput (Pawn|GetControlledPawn) AxisValue)))

(event Input|AxisEvents|InputAxisTurnRight/LeftMouse
  (params (AxisValue :type Float%20%28single-precision%29))
  (if (Variables|Default|GetCanMove)
    (Pawn|Input|AddControllerYawInput (Pawn|GetControlledPawn) AxisValue)))

(event Input|AxisEvents|InputAxisMoveBackward
  (params (AxisValue :type Float%20%28single-precision%29))
  (bind _returnvalue (Pawn|GetControlledPawn))
  ;[0.5034 1 0.92] Movements
  ;;[1 0.9233 0.156] Move Forward/Backward
  (if (Variables|Default|GetCanMove)
    (Pawn|Input|AddMovementInput _returnvalue (* AxisValue (Math|Vector|GetForwardVector (Pawn|GetControlRotation _returnvalue :!class /Script/Engine.Pawn))) (Variables|Default|GetMoveSpeed) false)))

(event Input|AxisEvents|InputAxisMoveRight
  (params (AxisValue :type Float%20%28single-precision%29))
  (bind _returnvalue (Pawn|GetControlledPawn))
  ;[0.5034 1 0.92] Movements
  ;;[1 0.4875 0.09621] Move Right/Left
  (if (Variables|Default|GetCanMove)
    (Pawn|Input|AddMovementInput _returnvalue (* AxisValue (Math|Vector|GetRightVector (Pawn|GetControlRotation _returnvalue :!class /Script/Engine.Pawn))) (Variables|Default|GetMoveSpeed) false)))

(event Input|AxisEvents|InputAxisMoveLeft
  (params (AxisValue :type Float%20%28single-precision%29))
  (bind _returnvalue (Pawn|GetControlledPawn))
  ;[0.5034 1 0.92] Movements
  ;;[1 0.4875 0.09621] Move Right/Left
  (if (Variables|Default|GetCanMove)
    (Pawn|Input|AddMovementInput _returnvalue (* AxisValue (Math|Vector|GetRightVector (Pawn|GetControlRotation _returnvalue :!class /Script/Engine.Pawn))) (Variables|Default|GetMoveSpeed) false)))

(fn ConstructionScript)