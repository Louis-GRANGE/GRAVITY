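; Level editor actor that auto-routes cables between two surface points received from the editor pawn's auto-generate spline event.
; FindBetterPath recursively builds an axis-aligned route, tracing along X, Y, then Z toward the target and stopping at hits.
; When blocked, GetNextFreePoint steps sideways with recursive traces to find a clearance around the obstacle.
; GenerateCableBySpline then adds a CableComponent per segment; debug traces, spheres and prints accompany generation.
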(event Custom|CustomEvent_0
  (params (FirstPoint :type Hit%20Result%20Structure) (LastPoint :type Hit%20Result%20Structure))
  (bind (_bblockinghit _binitialoverlap _time _distance _location _impactpoint _normal) (Collision|BreakHitResult LastPoint))
  (bind (_bblockinghit_2 _binitialoverlap_2 _time_2 _distance_2 _location_2 _impactpoint_2 _normal_2) (Collision|BreakHitResult FirstPoint))
  (Utilities|Array|Clear (Variables|Default|GetPoints))
  (Variables|Default|SetIteration 0)
  (CallFunction|FindBetterPath (+ _location_2 (* _normal_2 2e+01)) (+ _location (* _normal 2e+01)))
  (CallFunction|GenerateCablebySpline (Variables|Default|GetPoints))
  (Development|PrintString "GENERATE"))

(event EventBeginPlay
  (bind _asbp_level_editor__pawn (Utilities|Casting|CastToBP_LevelEditor-Pawn (Game|Player|GetPlayerPawn 0)))
  (bind _output_get (Variables|Default|SetAs%20BP%20Level%20Editor-%20Pawn _asbp_level_editor__pawn))
  (EventDispatchers|BindEventto+AutoGenerateSpline _output_get (delegate Custom|CustomEvent_0)))

(event Collision|EventActorBeginOverlap
  (params (OtherActor :type Actor%20Object%20Reference)))

(event EventTick
  (params (DeltaSeconds :type Float%20%28single-precision%29)))

(fn ConstructionScript)

(fn GenerateCablebySpline
  (params (Points :type Array%20of%20Vectors))
  (bind _returnvalue (Transformation|GetActorLocation))
  (Utilities|Array|Clear (Variables|Default|GetCables))
  (for _index (range 0 (- (Utilities|Array|Length Points) 2))
    (bind _returnvalue_2 (AddComponent|AddCableComponent false (Math|Transform|MakeTransform (- (Utilities|Array|Get(acopy) Points _index) _returnvalue) "0, 0,0.000000" "1.000000,1.000000,1.000000")))
    (Variables|/Script/CableComponent.CableComponent|SetEndLocation _returnvalue_2 (- (Utilities|Array|Get(acopy) Points (+ _index 1)) _returnvalue))
    (Variables|/Script/CableComponent.CableComponent|SetCableLength _returnvalue_2 (/ (Math|Vector|Distance(Vector) (Utilities|Array|Get(acopy) Points _index) (Utilities|Array|Get(acopy) Points (+ _index 1))) 1e+02))
    (Utilities|Array|Add (Variables|Default|GetCables) _returnvalue_2)))

(fn AddPointbyAxe
  (params (FirstPoint :type Vector) (LastPoint :type Vector) (Axe :type Vector) (NormalOffset :type Float%20%28single-precision%29))
  (bind _returnvalue (* LastPoint Axe))
  (bind _returnvalue_2 (- Axe 1.0))
  (bind _points (Variables|Default|GetPoints))
  (bind _points_2 (Variables|Default|GetPoints))
  (bind _points_3 (Variables|Default|GetPoints))
  (bind _returnvalue_3 (Utilities|Array|Length _points_3))
  (bind _returnvalue_4 (Utilities|Array|Length _points))
  (bind _returnvalue_5 (Math|Vector|VectorGetAbs _returnvalue_2))
  (bind _returnvalue_6 (- _returnvalue_3 1))
  (bind _returnvalue_7 (- _returnvalue_4 1))
  (bind _returnvalue_8 (* FirstPoint _returnvalue_5))
  (bind _output (Utilities|Array|Get(acopy) _points_3 _returnvalue_6))
  (bind _output_2 (Utilities|Array|Get(acopy) _points _returnvalue_7))
  (bind _returnvalue_9 (+ _returnvalue_8 _returnvalue))
  (bind (_outhit _returnvalue_10) (Collision|LineTraceByChannel FirstPoint _returnvalue_9 "TraceTypeQuery1" false 0 "ForDuration"))
  (if _returnvalue_10
    (if (Utilities|Operators|EqualEqual (+ (.Location (Collision|BreakHitResult _outhit)) (* (.Normal (Collision|BreakHitResult _outhit)) NormalOffset)) _output 1.0)
      (Development|PrintString "SAME POINT")
      (bind (_freepoint _havefound _movingtoaxe) (CallFunction|GetNextFreePoint _output_2 (CallFunction|GetBiggestfromVector (* (Math|Random|RandomUnitVector) _returnvalue_5)) Axe (* NormalOffset 2.0) 1e+01 0 10000 :!label _label))
      (if _havefound
        (Variables|Default|SetFree%20Point _freepoint)
        (else
          (bind (_freepoint_2 _havefound_2 _movingtoaxe_2) (CallFunction|GetNextFreePoint _output_2 (* _movingtoaxe -1.0) Axe (* NormalOffset 2.0) 1e+01 0 10000))
          (if _havefound_2
            (Variables|Default|SetFree%20Point _freepoint_2)
            (else
              (bind (_freepoint_3 _havefound_3 _movingtoaxe_3) (CallFunction|GetNextFreePoint "0, 0, 0" (Math|Vector|VectorGetAbs (- (+ (Math|Vector|VectorGetAbs _movingtoaxe_2) (Math|Vector|VectorGetAbs Axe)) 1.0)) Axe (* NormalOffset 2.0) 1e+01 0 10000))
              (if _havefound_3
                (Variables|Default|SetFree%20Point _freepoint_3)
                (else
                  (bind (_freepoint_4 _havefound_4) (CallFunction|GetNextFreePoint "0, 0, 0" (* _movingtoaxe_3 -1.0) Axe (* NormalOffset 2.0) 1e+01 0 10000))
                  (if _havefound_4
                    (Variables|Default|SetFree%20Point _freepoint_4)
                    (else
                      (goto _label)))))))))
      (Utilities|Array|Add (Variables|Default|GetPoints) (Variables|Default|GetFree%20Point))
      (Rendering|Debug|DrawDebugSphere (Variables|Default|GetFree%20Point) 5e+01 12 "(R=1.000000,G=0.000000,B=0.556560,A=1.000000)" 5e+01 2.0)
      (bind _end (CallFunction|AddPointbyAxe (Utilities|Array|Get(acopy) _points_2 (- (Utilities|Array|Length _points_2) 1)) LastPoint Axe NormalOffset))
      (return _end)
      (else
        (Utilities|Array|Add (Variables|Default|GetPoints) (+ (.Location (Collision|BreakHitResult _outhit)) (* (.Normal (Collision|BreakHitResult _outhit)) NormalOffset)))))
    (else
      (Utilities|Array|Add (Variables|Default|GetPoints) _returnvalue_9)))
  (return (Utilities|Operators|EqualEqual LastPoint _output 0.0)))

(fn FindBetterPath
  (params (FirstPoint :type Vector) (LastPoint :type Vector))
  (bind _points (Variables|Default|GetPoints))
  (bind _returnvalue (Utilities|Array|Length _points))
  (bind _returnvalue_2 (- _returnvalue 1))
  (bind _output (Utilities|Array|Get(acopy) _points _returnvalue_2))
  (bind _result (Math|Integer|IncrementInt (Variables|Default|GetIteration))
    (:%20%20
      (Development|PrintString (Utilities|String|ToString(Integer) _result))
      (Utilities|Array|Add (Variables|Default|GetPoints) FirstPoint)
      (bind _end (CallFunction|AddPointbyAxe _output LastPoint "1.000000, 0, 0" 2e+01))
      (if _end
        (return)
        (else
          (bind _end_2 (CallFunction|AddPointbyAxe _output LastPoint "0.000000,1.000000, 0" 2e+01))
          (if _end_2
            (return)
            (else
              (bind _end_3 (CallFunction|AddPointbyAxe _output LastPoint "0.000000,0.000000,1.000000" 2e+01))
              (if _end_3
                (return)
                (else
                  (CallFunction|FindBetterPath _output LastPoint))))))))))

(fn GetNextFreePoint
  (params (FirstPoint :type Vector) (AxeToMove :type Vector :default "0.000000,1.000000,0") (AxeToCheck :type Vector :default "1.000000,0,0") (NearlyIgnore :type Float%20%28double-precision%29) (Pas :type Float%20%28single-precision%29) (Iteration :type Integer) (MaxIteration :type Integer))
  (bind _returnvalue (* AxeToMove Pas))
  (bind _returnvalue_2 (+ FirstPoint _returnvalue))
  (if (< Iteration MaxIteration)
    (bind (_outhit _returnvalue_3) (Collision|LineTraceByChannel _returnvalue_2 (+ _returnvalue_2 (* AxeToCheck (* NearlyIgnore 2.0))) "TraceTypeQuery1" false 0 "ForDuration" true "(R=1.000000,G=0.000000,B=0.000000,A=1.000000)" "(R=0.000000,G=1.000000,B=0.000000,A=1.000000)" 2e+01))
    (if _returnvalue_3
      (if (> (.Distance (Collision|BreakHitResult _outhit)) NearlyIgnore)
        _
        (elif (Math|Float|NearlyEqual(Float) (.Distance (Collision|BreakHitResult _outhit)) 0.0 1e-06)
          (return "0, 0, 0" false AxeToMove)
          (else
            (bind (_freepoint _havefound) (CallFunction|GetNextFreePoint _returnvalue_2 AxeToMove AxeToCheck NearlyIgnore Pas (+ Iteration 1) MaxIteration))
            (return _freepoint _havefound AxeToMove)))))
    (return _returnvalue_2 true AxeToMove)
    (else
      (return "0, 0, 0" false AxeToMove))))