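; Singleton that serves as the game's online backend, using Google Sheets and Drive for per-level leaderboards, custom level lists and admin roles.
; VaRest HTTP calls read ranges through the Sheets API and send writes, searches and Drive file operations to a Google Apps Script.
; Init registers the Steam player and creates level pages with SORT formulas over PlayersData.
; Score submission keeps the best time; async responses chain through callback events and end in dispatchers.
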(event Custom|CustomEvent_0
  (params (Request :type Va%20Rest%20Request%20JSON%20Object%20Reference)))

(event Custom|CustomEvent_9
  (params (Request :type Va%20Rest%20Request%20JSON%20Object%20Reference))
  (bind _returnvalue (Class|VaRestRequestJSON|GetResponseObject Request))
  ;[0.3412 0.3012 1] Write in Scoreboard
  (bind _columname (Getter|GetColumnNamebyIndex (+ (Class|VaRestJsonObject|GetIntegerField _returnvalue "Column") 2)))
  (CallFunction|WriteinCell "PlayersData" _columname (Utilities|String|ToString(Integer) (Class|VaRestJsonObject|GetIntegerField _returnvalue "Row")) (Class|AdvancedIdentityLibrary|GetPlayerNickname (Class|AdvancedSteamFriendsLibrary|GetLocalSteamIDfromSteam)) (delegate Custom|CustomEvent_10)))

(event Custom|CustomEvent_16
  (params (Role :type E_Role%20Enum :default "NewEnumerator0")))

(event Custom|CustomEvent_11
  (params (Request :type Va%20Rest%20Request%20JSON%20Object%20Reference))
  ;[0.3412 0.3012 1] Write in Scoreboard
  (bind _columname (Getter|GetColumnNamebyIndex (Class|VaRestJsonObject|GetIntegerField (Class|VaRestRequestJSON|GetResponseObject Request) "Column")))
  (Getter|GetCellData "PlayersData" (Utilities|String|Append _columname (Utilities|String|ToString(Integer) (Class|VaRestJsonObject|GetIntegerField (Class|VaRestRequestJSON|GetResponseObject (stale Custom|Evt_OnFindCell Request)) "Row"))) (delegate Custom|Evt_GetPlayerTime)))

(event Custom|CustomEvent_10
  (params (Request :type Va%20Rest%20Request%20JSON%20Object%20Reference))
  ;[0.3412 0.3012 1] Write in Scoreboard
  (Getter|FindValueinSheet "PlayersData" (stale Custom|WriteInScoreboard Level) (delegate Custom|Evt_FindLevelColumn)))

(event Custom|GetAllTop100
  (Variables|Default|SetCurrentPage 0)
  (Getter|GetTop100OfLevel (Utilities|String|Append "Level_" (Utilities|String|ToString(Integer) (Variables|Default|GetCurrentPage))) "" (delegate Custom|Evt_ResponseGetTop100)))

(event Custom|Evt_ResponseGetTop100
  (params (Request :type Va%20Rest%20Request%20JSON%20Object%20Reference))
  (bind _returnvalue (Class|VaRestRequestJSON|GetResponseCode Request))
  (bind _currentpage (Variables|Default|GetCurrentPage))
  (bind _returnvalue_2 (Utilities|String|ToString(Integer) _currentpage))
  (bind _returnvalue_3 (== _returnvalue 200))
  (if (<= (Variables|Default|GetCurrentPage) (Variables|/Game/05_BP/GI_Gravity.GI_Gravity_C|GetNbLevels (.AsGI%20Gravity (Utilities|Casting|CastToGI_Gravity (Variables|Default|GetGameInstance)))))
    (if _returnvalue_3
      ;[1 1 1] AREVOIR
      (bind _playersdata (Getter|GetTop100Datas Request))
      (Utilities|Array|AppendArray (Variables|Default|GetPlayersData) _playersdata)
      (Math|Integer|IncrementInt (Variables|Default|GetCurrentPage)
        (:%20%20
          (Getter|GetTop100OfLevel (Utilities|String|Append "Level_" (Utilities|String|ToString(Integer) (Variables|Default|GetCurrentPage))) "" (delegate Custom|Evt_ResponseGetTop100))))
      (else
        (CallFunction|CreateNewPage _returnvalue_2 (delegate Custom|Evt_ResponseCreatePage))))
    (elif _returnvalue_3
      (CallFunction|DeletePage _returnvalue_2 (delegate Custom|CustomEvent_1))
      (else
        (Default|Call+OnPlayerDataLoaded self)))))

(event Custom|Evt_OnFindCell
  (params (Request :type Va%20Rest%20Request%20JSON%20Object%20Reference))
  ;[0.3412 0.3012 1] Write in Scoreboard
  (if (Class|VaRestJsonObject|GetBoolField (Class|VaRestRequestJSON|GetResponseObject Request) "IsFound")
    (Getter|FindValueinSheet "PlayersData" (stale Custom|WriteInScoreboard Level) (delegate Custom|CustomEvent_11))
    (else
      (CallFunction|WriteinFirstEmptyCellOfColumn "PlayersData" "SteamID" (Class|AdvancedSessionsLibrary|UniqueNetIdtoString (Class|AdvancedSteamFriendsLibrary|GetLocalSteamIDfromSteam)) (delegate Custom|CustomEvent_9)))))

(event Custom|CustomEvent_3
  (params (Request :type Va%20Rest%20Request%20JSON%20Object%20Reference)))

(event Custom|Call_GetAllCustomLevel
  ;[0.5211 0.2619 1] Get All Custom Level
  (Getter|GetDatas (Variables|Default|GetSheet%20ID) "CustomLevel" "A3" "C1000" (delegate Custom|CustomEvent_13)))

(event Custom|Evt_FindLevelColumn
  (params (Request :type Va%20Rest%20Request%20JSON%20Object%20Reference))
  ;[0.3412 0.3012 1] Write in Scoreboard
  (CallFunction|WriteinCell "PlayersData" (Utilities|String|ToString(Integer) (Class|VaRestJsonObject|GetIntegerField (Class|VaRestRequestJSON|GetResponseObject Request) "Column")) (Utilities|String|ToString(Integer) (Class|VaRestJsonObject|GetIntegerField (Class|VaRestRequestJSON|GetResponseObject (stale Custom|CustomEvent_9 Request)) "Row")) (Utilities|String|Replace (Utilities|String|ToString(Float) (stale Custom|WriteInScoreboard Time)) "." ",") (delegate Custom|CustomEvent_2)))

(event Custom|Evt_OnGetTop100OfLevel
  (params (Request :type Va%20Rest%20Request%20JSON%20Object%20Reference))
  ;[0.5211 0.2619 1] Top 100 Of Level
  (bind _playersdata (Getter|GetTop100Datas Request (stale Custom|Call_GetTop100OfLevel LevelID) (Class|VaRestJsonObject|GetIntegerField (Class|VaRestRequestJSON|GetResponseObject (stale Custom|CustomEvent_5 Request)) "ColumnIndex")))
  (Variables|Default|SetPlayersData _playersdata)
  (Default|Call+OnPlayerDataLoaded self))

(event Custom|CustomEvent_12
  (params (Request :type Va%20Rest%20Request%20JSON%20Object%20Reference))
  ;[0.8463 1 0.4316] To Download File on Drive and write it in the file
  (Class|BaseFilesDownloader|SaveArraytoFile (.Dest (Class|VaRestLibrary|Base64DecodeData (Variables|/Script/VaRest.VaRestRequestJSON|GetResponseContent Request))) "B:\\Projects\\UE4\\Gravity\\Saved\\SaveGames\\CustomMap\\SaveTree2.sav"))

(event Custom|Evt_GetPlayerTime
  (params (Request :type Va%20Rest%20Request%20JSON%20Object%20Reference))
  (bind _returnvalue (Class|VaRestRequestJSON|GetResponseObject Request))
  (bind _returnvalue_2 (Class|VaRestJsonObject|GetNumberField _returnvalue "Data"))
  ;[0.3412 0.3012 1] Write in Scoreboard
  (if (or (< (stale Custom|WriteInScoreboard Time) _returnvalue_2) (== _returnvalue_2 0.0))
    (CallFunction|WriteinCell "PlayersData" (stale Custom|CustomEvent_11 _columname) (Utilities|String|ToString(Integer) (Class|VaRestJsonObject|GetIntegerField (Class|VaRestRequestJSON|GetResponseObject (stale Custom|Evt_OnFindCell Request)) "Row")) (Utilities|String|Replace (Utilities|String|ToString(Float) (stale Custom|WriteInScoreboard Time)) "." ",") (delegate Custom|CustomEvent))
    (else
      (Default|Call+OnWriteinScoreboardFinish _returnvalue_2 (stale Custom|WriteInScoreboard Time)))))

(event Custom|CustomEvent_2
  (params (Request :type Va%20Rest%20Request%20JSON%20Object%20Reference))
  ;[0.3412 0.3012 1] Write in Scoreboard
  (Default|Call+OnWriteinScoreboardFinish (stale Custom|WriteInScoreboard Time) (stale Custom|WriteInScoreboard Time)))

(event Custom|Call_GetTop100OfLevel
  (params (LevelID :type String))
  ;[0.5211 0.2619 1] Top 100 Of Level
  (Getter|GetColumnbyName "PlayersData" LevelID (delegate Custom|CustomEvent_5)))

(event Custom|CustomEvent_5
  (params (Request :type Va%20Rest%20Request%20JSON%20Object%20Reference))
  (bind _returnvalue (Class|VaRestRequestJSON|GetResponseObject Request))
  ;[0.5211 0.2619 1] Top 100 Of Level
  (if (Class|VaRestJsonObject|GetBoolField _returnvalue "IsFound")
    (Getter|GetTop100OfLevel (stale Custom|Call_GetTop100OfLevel LevelID) (Class|VaRestJsonObject|GetStringField _returnvalue "ColumnLetter") (delegate Custom|Evt_OnGetTop100OfLevel))))

(event Custom|CustomEvent_13
  (params (Request :type Va%20Rest%20Request%20JSON%20Object%20Reference))
  ;[0.5211 0.2619 1] Get All Custom Level
  (bind _customlevelsdata (Getter|GetAllCustomLevelDatas Request))
  (Variables|Default|SetCustomLevels _customlevelsdata)
  (Default|Call+OnCustomLevelDataLoaded self))

(event Custom|Evt_ResponseCreatePage
  (params (Request :type Va%20Rest%20Request%20JSON%20Object%20Reference))
  (Math|Integer|IncrementInt (Variables|Default|GetCurrentPage)
    (:%20%20
      (Getter|GetTop100OfLevel (Utilities|String|Append "Level_" (Utilities|String|ToString(Integer) (Variables|Default|GetCurrentPage))) "" (delegate Custom|Evt_ResponseGetTop100)))))

(event Custom|CustomEvent_1
  (params (Request :type Va%20Rest%20Request%20JSON%20Object%20Reference))
  (if (== (Class|VaRestRequestJSON|GetResponseCode Request) 200)
    (Math|Integer|IncrementInt (Variables|Default|GetCurrentPage)
      (:%20%20
        (Getter|GetTop100OfLevel (Utilities|String|Append "Level_" (Utilities|String|ToString(Integer) (Variables|Default|GetCurrentPage))) "" (delegate Custom|Evt_ResponseGetTop100))))))

(event Custom|CustomEvent_4
  (params (Request :type Va%20Rest%20Request%20JSON%20Object%20Reference))
  (CallFunction|GenerateRandomData (stale Custom|GenerateRandomData NbToGenerate) (+ (stale Custom|GenerateRandomData Current) 1) (stale Custom|GenerateRandomData StartAtLine)))

(event Custom|WriteInScoreboard
  (params (Level :type String) (Time :type Float%20%28double-precision%29))
  ;[0.3412 0.3012 1] Write in Scoreboard
  (Getter|FindValueinSheet "PlayersData" (Class|AdvancedSessionsLibrary|UniqueNetIdtoString (Class|AdvancedSteamFriendsLibrary|GetLocalSteamIDfromSteam)) (delegate Custom|Evt_OnFindCell)))

(event Custom|GenerateRandomData
  (params (NbToGenerate :type Integer) (Current :type Integer) (StartAtLine :type Integer))
  (bind _returnvalue (+ Current StartAtLine))
  (bind _returnvalue_2 (Utilities|String|ToString(Integer) _returnvalue))
  (if (>= NbToGenerate Current)
    (bind _output (Getter|GetRandomString (Math|Random|RandomIntegerinRange 4 20) true true true))
    (CallFunction|WriteinCell "1" "A" _returnvalue_2 _output (delegate Custom|CustomEvent_0))
    (CallFunction|WriteinCell "1" "B" _returnvalue_2 (Utilities|String|ToString(Integer) (Utilities|String|Len _output)) (delegate Custom|CustomEvent_4))
    (else
      (CallFunction|SortDataatPage "1" "A" "0" "B" "101" 2 (delegate Custom|CustomEvent_3)))))

(event Custom|CustomEvent
  (params (Request :type Va%20Rest%20Request%20JSON%20Object%20Reference))
  ;[0.3412 0.3012 1] Write in Scoreboard
  (Default|Call+OnWriteinScoreboardFinish (Class|VaRestJsonObject|GetNumberField (Class|VaRestRequestJSON|GetResponseObject (stale Custom|Evt_GetPlayerTime Request)) "Data") (stale Custom|WriteInScoreboard Time)))

(event EventInit
  (|CallParentFunction)
  (CallFunction|SetupPlayerData)
  (CallFunction|CreateLevelPage)
  (Admin|GetRole (delegate Custom|CustomEvent_16)))

(event Custom|SetupPlayerData
  ;[1 0.5021 0.939] Create Data Player with the Steam ID
  (Getter|FindValueinSheet "PlayersData" (Class|AdvancedSessionsLibrary|UniqueNetIdtoString (Class|AdvancedSteamFriendsLibrary|GetLocalSteamIDfromSteam)) (delegate Custom|Evt_FindPlayerData)))

(event Custom|Evt_WirtePlayerSteamID
  (params (Request :type Va%20Rest%20Request%20JSON%20Object%20Reference))
  (bind _returnvalue (Class|VaRestRequestJSON|GetResponseObject Request))
  ;[1 0.5021 0.939] Create Data Player with the Steam ID
  (bind _columname (Getter|GetColumnNamebyIndex (+ (Class|VaRestJsonObject|GetIntegerField _returnvalue "Column") 1)))
  (CallFunction|WriteinCell "PlayersData" _columname (Utilities|String|ToString(Integer) (Class|VaRestJsonObject|GetIntegerField _returnvalue "Row")) (Class|AdvancedIdentityLibrary|GetPlayerNickname (Class|AdvancedSteamFriendsLibrary|GetLocalSteamIDfromSteam)) (delegate Custom|CustomEvent_6)))

(event Custom|CustomEvent_8
  (params (Request :type Va%20Rest%20Request%20JSON%20Object%20Reference))
  (if (<= (Variables|Default|GetCurrentPage) (Variables|/Game/05_BP/GI_Gravity.GI_Gravity_C|GetNbLevels (.AsGI%20Gravity (Utilities|Casting|CastToGI_Gravity (Variables|Default|GetGameInstance)))))
    (Math|Integer|IncrementInt (Variables|Default|GetCurrentPage)
      (:%20%20
        (CallFunction|CreatePageifNotExiste (Utilities|String|Append "Level_" (Utilities|String|ToString(Integer) (Variables|Default|GetCurrentPage))) (delegate Custom|Evt_Response-CreatePageIfNorExist))))))

(event Custom|Evt_FindPlayerData
  (params (Request :type Va%20Rest%20Request%20JSON%20Object%20Reference))
  ;[1 0.5021 0.939] Create Data Player with the Steam ID
  (if (not (Class|VaRestJsonObject|GetBoolField (Class|VaRestRequestJSON|GetResponseObject Request) "IsFound"))
    (CallFunction|WriteinFirstEmptyCellOfColumn "PlayersData" "SteamID" (Class|AdvancedSessionsLibrary|UniqueNetIdtoString (Class|AdvancedSteamFriendsLibrary|GetLocalSteamIDfromSteam)) (delegate Custom|Evt_WirtePlayerSteamID))))

(event Custom|CreateLevelPage
  (Variables|Default|SetCurrentPage 0)
  (CallFunction|CreatePageifNotExiste (Utilities|String|Append "Level_" (Utilities|String|ToString(Integer) (Variables|Default|GetCurrentPage))) (delegate Custom|Evt_Response-CreatePageIfNorExist)))

(event Custom|Evt_Response-CreatePageIfNorExist
  (params (Request :type Va%20Rest%20Request%20JSON%20Object%20Reference))
  (bind _columname (Getter|GetColumnNamebyIndex (+ (Variables|Default|GetCurrentPage) (Variables|Default|GetColumnPayerDataOffset))))
  (CallFunction|WriteinCell (Utilities|String|ToString(Integer) (Variables|Default|GetCurrentPage)) "A" "2" (Utilities|String|ToString(Text) (Utilities|Text|FormatText "=SORT(PlayersData!A2:{Level};PlayersData!{Level}2:{Level};1)" _columname)) (delegate Custom|CustomEvent_7)))

(event Custom|CustomEvent_6
  (params (Request :type Va%20Rest%20Request%20JSON%20Object%20Reference))
  ;[1 0.5021 0.939] Create Data Player with the Steam ID
)

(event Custom|CustomEvent_7
  (params (Request :type Va%20Rest%20Request%20JSON%20Object%20Reference))
  (CallFunction|WriteinCell "PlayersData" (stale Custom|Evt_Response-CreatePageIfNorExist _columname) "1" (Utilities|String|ToString(Text) (Utilities|Text|FormatText "Level_{LevelIndex}" (Variables|Default|GetCurrentPage))) (delegate Custom|CustomEvent_8)))

(event Custom|Call_GetAllAdmins
  (Getter|GetDatas (Variables|Default|GetSheet%20ID) "Admin" "A2" "C101" (delegate Custom|CustomEvent_17)))

(event Custom|CustomEvent_17
  (params (Request :type Va%20Rest%20Request%20JSON%20Object%20Reference))
  (bind _alladmin (Admin|GetAllAdmins Request))
  (Variables|Default|SetPlayersAdminData _alladmin)
  (Default|Call+OnPlayerAdminDataLoaded self))

(event Custom|CustomEvent_15
  (params (Request :type Va%20Rest%20Request%20JSON%20Object%20Reference))
  (bind _returnvalue (Class|VaRestRequestJSON|GetResponseObject Request))
  (bind _returnvalue_2 (Class|VaRestJsonObject|GetIntegerField _returnvalue "Data"))
  (bind _returnvalue_3 (Math|Conversions|ToByte(Integer) _returnvalue_2))
  (bind _returnvalue_4 (Utilities|Enum|ByteToEnumE_Role _returnvalue_3))
  ;[0.5426 0.2648 1] Get Admin Role
  (Variables|Default|SetRole _returnvalue_4)
  (Default|Call+GetRole _returnvalue_4))

(event Custom|Call_GetRole
  ;[0.5426 0.2648 1] Get Admin Role
  (Getter|FindValueinSheet "Admin" (Class|AdvancedSessionsLibrary|UniqueNetIdtoString (Class|AdvancedSteamFriendsLibrary|GetLocalSteamIDfromSteam)) (delegate Custom|CustomEvent_14)))

(event Custom|CustomEvent_14
  (params (Request :type Va%20Rest%20Request%20JSON%20Object%20Reference))
  (bind _returnvalue (Class|VaRestRequestJSON|GetResponseObject Request))
  ;[0.5426 0.2648 1] Get Admin Role
  (if (Class|VaRestJsonObject|GetBoolField _returnvalue "IsFound")
    (Getter|GetCellData "Admin" (Utilities|String|Append "C" (Utilities|String|ToString(Integer) (Class|VaRestJsonObject|GetIntegerField _returnvalue "Row"))) (delegate Custom|CustomEvent_15))
    (else
      (Variables|Default|SetRole "NewEnumerator2")
      (Default|Call+GetRole "NewEnumerator2"))))

(fn GetDatas
  (params (SheetID :type String) (SheetName :type String) (CellA :type String) (CellB :type String) (Response :type Delegate%20%28by%20ref%29))
  (Class|VaRestSubsystem|CallURL (|VaRestSubsystem) (Utilities|String|ToString(Text) (Utilities|Text|FormatText "https://sheets.googleapis.com/v4/spreadsheets/{SheetID}/values/{SheetName}!{CellA}:{CellB}?key={APIKey}" SheetID SheetName CellA CellB (Variables|Default|GetAPIKey))) "GET" "x_www_form_urlencoded_url" 0 Response))

(fn GetTop100OfLevel
  (params (LevelID :type String) (ColumnLetter :type String) (Response :type Delegate%20%28by%20ref%29))
  (Getter|GetDatas (Variables|Default|GetSheet%20ID) LevelID "A2" (Utilities|String|ToString(Text) (Utilities|Text|FormatText "{IndexLevel}101" ColumnLetter)) Response))

(fn CreateNewPage
  (params (PageName :type String) (Response :type Delegate%20%28by%20ref%29))
  (Class|VaRestSubsystem|CallURL (|VaRestSubsystem) (Utilities|String|ToString(Text) (Utilities|Text|FormatText "https://script.google.com/macros/s/{DeploimentID}/exec?FunctionName=CreateSheetPage&NewPageName={PageName}&SheetID={SheetID}" (Variables|Default|GetDeploimentID) PageName (Variables|Default|GetSheet%20ID))) "POST" "x_www_form_urlencoded_url" 0 Response))

(fn DeletePage
  (params (PageName :type String) (Response :type Delegate%20%28by%20ref%29))
  (Class|VaRestSubsystem|CallURL (|VaRestSubsystem) (Utilities|String|ToString(Text) (Utilities|Text|FormatText "https://script.google.com/macros/s/{DeploimentID}/exec?FunctionName=DeleteSheetPage&PageToDelete={PageName}&SheetID={SheetID}" (Variables|Default|GetDeploimentID) PageName (Variables|Default|GetSheet%20ID))) "POST" "x_www_form_urlencoded_url" 0 Response))

(fn GetTop100Datas
  (params (Response :type Va%20Rest%20Request%20JSON%20Object%20Reference) (LevelID :type String) (ColumnIndex :type Integer))
  (for _array_element (Class|VaRestJsonObject|GetArrayField (Class|VaRestRequestJSON|GetResponseObject Response) "values")
    (Utilities|Array|Add (LocalVariables|GetPlayersDataOfLevel) (Utilities|Struct|MakeS_PlayerData (Class|VaRestJsonValue|AsString (Utilities|Array|Get(acopy) (Class|VaRestJsonValue|AsArray _array_element) 1)) (Class|VaRestJsonValue|AsString (Utilities|Array|Get(acopy) (Class|VaRestJsonValue|AsArray _array_element))) (Class|VaRestJsonValue|AsString (Utilities|Array|Get(acopy) (Class|VaRestJsonValue|AsArray _array_element) (- ColumnIndex 1))) LevelID)))
  (return (LocalVariables|GetPlayersDataOfLevel)))

(fn SortDataatPage
  (params (PageName :type String) (FromCol :type String) (FromLine :type String) (ToCol :type String) (ToLine :type String) (SortCol :type Integer) (Response :type Delegate%20%28by%20ref%29))
  (Class|VaRestSubsystem|CallURL (|VaRestSubsystem) (Utilities|String|ToString(Text) (Utilities|Text|FormatText "https://script.google.com/macros/s/{DeploimentID}/exec?FunctionName=SortByColumn&SheetID={SheetID}&PageName={PageName}&CellA={FromColl}{FromLine}&CellB={ToCol}{ToLine}&SortCol={SortCol}" (Variables|Default|GetDeploimentID) (Variables|Default|GetSheet%20ID) PageName FromCol FromLine ToCol ToLine SortCol)) "POST" "x_www_form_urlencoded_url" 0 Response))

(fn WriteinCell
  (params (PageName :type String) (AtCol :type String) (AtLine :type String) (Value :type String) (Response :type Delegate%20%28by%20ref%29))
  (Class|VaRestSubsystem|CallURL (|VaRestSubsystem) (Utilities|String|ToString(Text) (Utilities|Text|FormatText "https://script.google.com/macros/s/{DeploimentID}/exec?FunctionName=WriteInCell&SheetID={SheetID}&PageName={PageName}&Cell={Col}{Line}&Value={Value}" (Variables|Default|GetDeploimentID) (Variables|Default|GetSheet%20ID) PageName AtCol AtLine (Class|VaRestLibrary|PercentEncode Value))) "POST" "x_www_form_urlencoded_url" 0 Response))

(fn GetRandomString
  (params (Size :type Integer) (UseAlphabet :type Boolean) (UseNumeric :type Boolean) (UseSpecial :type Boolean))
  (bind _gameinstance (Variables|Default|GetGameInstance))
  (bind _asgi_gravity (Utilities|Casting|CastToGI_Gravity _gameinstance))
  (for _index (range 0 (- Size 1))
    (LocalVariables|SetOut (Utilities|String|Append (LocalVariables|GetOut) (.OutItem (Utilities|Array|Random (Utilities|String|GetCharacterArrayfromString (Utilities|String|Append (select UseAlphabet (Default|GetAlphabet _asgi_gravity) "") (select UseNumeric (Default|GetNumeric _asgi_gravity) "") (select UseSpecial (Default|GetSymbol _asgi_gravity) ""))))))))
  (return (LocalVariables|GetOut)))

(fn FindValueinSheet
  (params (PageName :type String) (TextToFind :type String) (Response :type Delegate%20%28by%20ref%29))
  (Class|VaRestSubsystem|CallURL (|VaRestSubsystem) (Utilities|String|ToString(Text) (Utilities|Text|FormatText "https://script.google.com/macros/s/{DeploimentID}/exec?FunctionName=FindCellInPage&SheetID={SheetID}&PageName={PageName}&TextToFind={TextToFind}" (Variables|Default|GetDeploimentID) (Variables|Default|GetSheet%20ID) PageName (Class|VaRestLibrary|PercentEncode TextToFind))) "POST" "x_www_form_urlencoded_url" 0 Response))

(fn GetTop100OfLevel
  (params (OnDataLoaded :type Delegate%20%28by%20ref%29) (LevelID :type String))
  (EventDispatchers|BindEventto+OnPlayerDataLoaded OnDataLoaded)
  (CallFunction|CallGetTop100OfLevel LevelID))

(fn GetColumnNamebyIndex
  (params (ColumnIndex :type Integer))
  (if (<= ColumnIndex 0)
    (return "")
    (else
      (LocalVariables|SetIndex ColumnIndex)
      (bind _asgi_gravity (Utilities|Casting|CastToGI_Gravity (Variables|Default|GetGameInstance)))
      (while (> (LocalVariables|GetIndex) 0)
        (LocalVariables|SetColumName_Tmp (Utilities|String|Append (Utilities|Array|Get(acopy) (Utilities|String|GetCharacterArrayfromString (Default|GetAlphabet _asgi_gravity)) (Math|Integer|%(Integer) (- (LocalVariables|GetIndex) 1) 26)) (LocalVariables|GetColumName_Tmp)))
        (LocalVariables|SetIndex (Math|Float|Floor (/ (Math|Conversions|ToFloat(Integer) (- (LocalVariables|GetIndex) 1)) 26.0))))
      (return (Class|KismetStringLibrary|ToUpper (LocalVariables|GetColumName_Tmp))))))

(fn WriteinFirstEmptyCellOfColumn
  (params (PageName :type String) (ColumnName :type String) (Value :type String) (Response :type Delegate%20%28by%20ref%29))
  (Class|VaRestSubsystem|CallURL (|VaRestSubsystem) (Utilities|String|ToString(Text) (Utilities|Text|FormatText "https://script.google.com/macros/s/{DeploimentID}/exec?FunctionName=WriteInFirstEmptyCellOfColumn&SheetID={SheetID}&PageName={PageName}&ColumnName={ColumnName}&Value={Value}" (Variables|Default|GetDeploimentID) (Variables|Default|GetSheet%20ID) PageName ColumnName (Class|VaRestLibrary|PercentEncode Value))) "POST" "x_www_form_urlencoded_url" 0 Response))

(fn CreatePageifNotExiste
  (params (PageName :type String) (Response :type Delegate%20%28by%20ref%29))
  (Class|VaRestSubsystem|CallURL (|VaRestSubsystem) (Utilities|String|ToString(Text) (Utilities|Text|FormatText "https://script.google.com/macros/s/{DeploimentID}/exec?FunctionName=CreatePageIfNotExiste&PageName={PageName}&SheetID={SheetID}" (Variables|Default|GetDeploimentID) PageName (Variables|Default|GetSheet%20ID))) "POST" "x_www_form_urlencoded_url" 0 Response))

(fn GetCellData
  (params (PageName :type String) (Cell :type String) (Response :type Delegate%20%28by%20ref%29))
  (Class|VaRestSubsystem|CallURL (|VaRestSubsystem) (Utilities|String|ToString(Text) (Utilities|Text|FormatText "https://script.google.com/macros/s/{DeploimentID}/exec?FunctionName=GetDataCell&SheetID={SheetID}&PageName={PageName}&Cell={Cell}" (Variables|Default|GetDeploimentID) (Variables|Default|GetSheet%20ID) PageName Cell)) "POST" "x_www_form_urlencoded_url" 0 Response))

(fn WriteinFirstEmptyCellOfLine
  (params (PageName :type String) (Line :type String) (Value :type String) (Response :type Delegate%20%28by%20ref%29))
  (Class|VaRestSubsystem|CallURL (|VaRestSubsystem) (Utilities|String|ToString(Text) (Utilities|Text|FormatText "https://script.google.com/macros/s/{DeploimentID}/exec?FunctionName=WriteInFirstEmptyCellOfLine&SheetID={SheetID}&PageName={PageName}&Line={Line}&Value={Value}" (Variables|Default|GetDeploimentID) (Variables|Default|GetSheet%20ID) PageName Line (Class|VaRestLibrary|PercentEncode Value))) "POST" "x_www_form_urlencoded_url" 0 Response))

(fn GetColumnbyName
  (params (PageName :type String) (ColumnName :type String) (Response :type Delegate%20%28by%20ref%29))
  (Class|VaRestSubsystem|CallURL (|VaRestSubsystem) (Utilities|String|ToString(Text) (Utilities|Text|FormatText "https://script.google.com/macros/s/{DeploimentID}/exec?FunctionName=GetColumnByName&SheetID={SheetID}&PageName={PageName}&ColumnName={ColumnName}" (Variables|Default|GetDeploimentID) (Variables|Default|GetSheet%20ID) PageName ColumnName)) "POST" "x_www_form_urlencoded_url" 0 Response))

(fn UploadFileonDrive
  (params (Path :type String) (RequestFinish :type Delegate%20%28by%20ref%29) (FileName :type String) (Override :type Boolean))
  (bind (_result _returnvalue) (Class|BaseFilesDownloader|LoadFiletoArray Path))
  (if _returnvalue
    (bind _returnvalue_2 (Class|VaRestSubsystem|ConstructVaRestRequestExt (|VaRestSubsystem) "POST" "binary"))
    (LocalVariables|SetRequest _returnvalue_2)
    (Class|VaRestRequestJSON|SetHeader (LocalVariables|GetRequest) "Content-Type" "application/octet-stream")
    (Class|VaRestRequestJSON|SetBinaryRequestContent (LocalVariables|GetRequest) _result)
    (EventDispatchers|BindEventtoOnRequestComplete (LocalVariables|GetRequest) RequestFinish)
    (EventDispatchers|BindEventtoOnRequestFail (LocalVariables|GetRequest) RequestFinish)
    (Class|VaRestRequestJSON|ProcessURL (LocalVariables|GetRequest) (Utilities|String|ToString(Text) (Utilities|Text|FormatText "https://script.google.com/macros/s/{DeploimentID}/exec?FunctionName=UploadFileToDrive&FolderId={FolderID}&FileName={FileName}&Override={Override}" (Variables|Default|GetDeploimentID) (Variables|Default|GetFolderID) FileName Override)))))

(fn DownloadFileonDrive
  (params (FileName :type String) (Response :type Delegate%20%28by%20ref%29))
  (bind _returnvalue (Class|VaRestSubsystem|ConstructVaRestRequestExt (|VaRestSubsystem) "GET" "x_www_form_urlencoded_url"))
  (Class|VaRestRequestJSON|SetHeader _returnvalue "Content-Type" "application/octet-stream")
  (EventDispatchers|BindEventtoOnRequestFail _returnvalue Response)
  (EventDispatchers|BindEventtoOnRequestComplete _returnvalue Response)
  (Class|VaRestRequestJSON|ProcessURL _returnvalue (Utilities|String|ToString(Text) (Utilities|Text|FormatText "https://script.google.com/macros/s/{DeploimentID}/exec?FunctionName=DownloadFileByName&FileName={FileName}" (Variables|Default|GetDeploimentID) FileName))))

(fn GetAllCustomLevelDatas
  (params (Response :type Va%20Rest%20Request%20JSON%20Object%20Reference))
  (for _array_element (Class|VaRestJsonObject|GetArrayField (Class|VaRestRequestJSON|GetResponseObject Response) "values")
    (Utilities|Array|Add (LocalVariables|GetPlayersDataOfLevel) (Utilities|Struct|MakeS_CustomLevelData (Class|VaRestJsonValue|AsString (Utilities|Array|Get(acopy) (Class|VaRestJsonValue|AsArray _array_element))) (Class|VaRestJsonValue|AsString (Utilities|Array|Get(acopy) (Class|VaRestJsonValue|AsArray _array_element) 1)) (Class|VaRestJsonValue|AsString (Utilities|Array|Get(acopy) (Class|VaRestJsonValue|AsArray _array_element) 2)) false)))
  (return (LocalVariables|GetPlayersDataOfLevel)))

(fn GetAllCustomLevels
  (params (OnDataLoaded :type Delegate%20%28by%20ref%29))
  (EventDispatchers|BindEventto+OnCustomLevelDataLoaded OnDataLoaded)
  (CallFunction|CallGetAllCustomLevel))

(fn GetRole
  (params (Response :type Delegate%20%28by%20ref%29))
  (EventDispatchers|BindEventto+GetRole Response)
  (CallFunction|CallGetRole))

(fn GetRolebyString
  (params (In :type String))
  (bind _enumvalue (|ForEachE_Role)
    (:LoopBody
      (if (Utilities|Enum|Equal(Enum) (Utilities|String|EnumtoString _enumvalue) In)
        (return _enumvalue)))
    (:then
      (return "NewEnumerator2"))))

(fn GetAllAdmins
  (params (Target :type Va%20Rest%20Request%20JSON%20Object%20Reference))
  (for _array_element (Class|VaRestJsonObject|GetArrayField (Class|VaRestRequestJSON|GetResponseObject Target) "values")
    (Utilities|Array|Add (LocalVariables|GetTmpPlayersAdminData) (Utilities|Struct|MakeS_PlayerAdminData (Class|VaRestJsonValue|AsString (Utilities|Array|Get(acopy) (Class|VaRestJsonValue|AsArray _array_element))) (Class|VaRestJsonValue|AsString (Utilities|Array|Get(acopy) (Class|VaRestJsonValue|AsArray _array_element) 1)) (Utilities|Enum|ByteToEnumE_Role (Math|Conversions|ToByte(Integer) (Class|VaRestJsonValue|AsInt32 (Utilities|Array|Get(acopy) (Class|VaRestJsonValue|AsArray _array_element) 2)))))))
  (return (LocalVariables|GetTmpPlayersAdminData)))

(fn GetAllAdmins
  (params (OnDataLoaded :type Delegate%20%28by%20ref%29))
  (EventDispatchers|BindEventto+OnPlayerAdminDataLoaded OnDataLoaded)
  (CallFunction|CallGetAllAdmins))

(fn CanSetRole?
  (params (NewRole :type E_Role%20Enum :default "NewEnumerator2"))
  (return (>= (Math|Conversions|ToInteger(Byte) (Variables|Default|GetRole)) (Math|Conversions|ToInteger(Byte) NewRole))))

(fn DeleteColumnbyName
  (params (PageName :type String) (ColumnName :type String) (Response :type Delegate%20%28by%20ref%29))
  (Class|VaRestSubsystem|CallURL (|VaRestSubsystem) (Utilities|String|ToString(Text) (Utilities|Text|FormatText "https://script.google.com/macros/s/{DeploimentID}/exec?FunctionName=DeleteColumnByName&SheetID={SheetID}&PageName={PageName}&ColumnName={ColumnName}" (Variables|Default|GetDeploimentID) (Variables|Default|GetSheet%20ID) PageName ColumnName)) "POST" "x_www_form_urlencoded_url" 0 Response))

(fn DeletePagebyName
  (params (PageName :type String) (Response :type Delegate%20%28by%20ref%29))
  (Class|VaRestSubsystem|CallURL (|VaRestSubsystem) (Utilities|String|ToString(Text) (Utilities|Text|FormatText "https://script.google.com/macros/s/{DeploimentID}/exec?FunctionName=DeletePageByName&SheetID={SheetID}&PageName={PageName}" (Variables|Default|GetDeploimentID) (Variables|Default|GetSheet%20ID) PageName)) "POST" "x_www_form_urlencoded_url" 0 Response))

(fn DeleteFilebyName
  (params (FileName :type String) (Response :type Delegate%20%28by%20ref%29))
  (Class|VaRestSubsystem|CallURL (|VaRestSubsystem) (Utilities|String|ToString(Text) (Utilities|Text|FormatText "https://script.google.com/macros/s/{DeploimentID}/exec?FunctionName=DeleteFileByName&FolderId={FolderId}&FileName={FileName}" (Variables|Default|GetDeploimentID) (Variables|Default|GetFolderID) FileName)) "POST" "x_www_form_urlencoded_url" 0 Response))

(fn DeleteRowbyIndex
  (params (PageName :type String) (Response :type Delegate%20%28by%20ref%29) (Row :type Integer))
  (Class|VaRestSubsystem|CallURL (|VaRestSubsystem) (Utilities|String|ToString(Text) (Utilities|Text|FormatText "https://script.google.com/macros/s/{DeploimentID}/exec?FunctionName=DeleteRow&SheetID={SheetID}&PageName={PageName}&RowIndex={Row}" (Variables|Default|GetDeploimentID) (Variables|Default|GetSheet%20ID) PageName Row)) "POST" "x_www_form_urlencoded_url" 0 Response))