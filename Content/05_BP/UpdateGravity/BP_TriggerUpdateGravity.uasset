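; Box trigger volume that applies its own gravity data to overlapping actors through UpdateGravityMessage.
; It tracks actors inside and hands them the global current gravity direction from the gravity game-state object when they leave.
; On a global gravity change matching certain ApplyTo targets, it re-sends its data to those inside after a short delay.
; The construction script sizes the box, decal and Niagara effect, coloring both visuals by gravity direction.
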(event OnComponentBeginOverlap(Box)
  (params (OverlappedComponent :type Primitive%20Component%20Object%20Reference) (OtherActor :type Actor%20Object%20Reference) (OtherComp :type Primitive%20Component%20Object%20Reference) (OtherBodyIndex :type Integer) (bFromSweep :type Boolean) (SweepResult :type Hit%20Result%20Structure%20%28by%20ref%29))
  (Class|BPIGravity|UpdateGravity(Message) OtherActor (Variables|Default|GetGravityData))
  (Utilities|Array|AddUnique (Variables|Default|GetActorsInside) OtherActor))

(event OnComponentEndOverlap(Box)
  (params (OverlappedComponent :type Primitive%20Component%20Object%20Reference) (OtherActor :type Actor%20Object%20Reference) (OtherComp :type Primitive%20Component%20Object%20Reference) (OtherBodyIndex :type Integer))
  (bind _gravitydata (Variables|Default|GetGravityData))
  (bind (_applyto _direction _scale _location _duration _sender) (Utilities|Struct|BreakS_GravityData _gravitydata))
  (Utilities|Array|RemoveItem (Variables|Default|GetActorsInside) OtherActor)
  (Class|BPIGravity|UpdateGravity(Message) OtherActor (Utilities|Struct|MakeS_GravityData _applyto (Variables|/Game/05_BP/GS_Gravity.GS_Gravity_C|GetCurrentApplyGravity (CallFunction|GetGSGravity)) _scale _location _duration _sender)))

(event Custom|Evt_OnGravityChange
  (params (Data :type S%20Gravity%20Data%20Structure))
  (bind _applyto (Utilities|Struct|BreakS_GravityData Data))
  (bind _ns_gravityeffect (Variables|Default|GetNS_GravityEffect))
  (bind _gravitydata (Variables|Default|GetGravityData))
  (bind _direction (Utilities|Struct|BreakS_GravityData _gravitydata))
  (Utilities|FlowControl|Delay 0.1)
  (if (or (Utilities|Array|ContainsItem _applyto "NewEnumerator3") (Utilities|Array|ContainsItem _applyto "NewEnumerator1"))
    (for _array_element (Variables|Default|GetActorsInside)
      (Class|BPIGravity|UpdateGravity(Message) _array_element _gravitydata))
    (Utilities|FlowControl|Delay 0.2)
    (Effects|Components|ParticleSystem|SetVectorParameter _ns_gravityeffect "GravityDirection" _direction)
    (bind _returnvalue (CallFunction|GetGravityColor _direction))
    (Niagara|SetNiagaraVariable(LinearColor) _ns_gravityeffect "GravityColor" _returnvalue)))

(event EventBeginPlay
  (Utilities|Struct|SetmembersinS_GravityData (Variables|Default|GetGravityData) (Transformation|GetActorLocation) self)
  (EventDispatchers|BindEventtoOnGravityChange (CallFunction|GetGSGravity) (delegate Custom|Evt_OnGravityChange))
  (CallFunction|SetMaterialData))

(event EventTick
  (params (DeltaSeconds :type Float%20%28single-precision%29)))

(fn ConstructionScript
  (CallFunction|Init))

(fn Init
  (Components|Box|SetBoxExtent (Variables|Default|GetBox) (Variables|Default|GetBoxExtend) true)
  (Transformation|SetRelativeScale3D (Variables|Default|GetDecal) (/ (Variables|Default|GetBoxExtend) 1e+02))
  (bind _returnvalue (Rendering|Material|CreateDynamicMaterialInstance (Variables|Default|GetDecal) :!class /Script/Engine.DecalComponent))
  (bind _output_get (Variables|Default|SetDecalMaterialInstance _returnvalue))
  (Rendering|Components|Decal|SetDecalMaterial (Variables|Default|GetDecal) _output_get)
  (CallFunction|SetMaterialData))

(fn SetMaterialData
  (bind _ns_gravityeffect (Variables|Default|GetNS_GravityEffect))
  (bind _gravitydata (Variables|Default|GetGravityData))
  (bind _direction (Utilities|Struct|BreakS_GravityData _gravitydata))
  (bind _returnvalue (CallFunction|GetGravityColor _direction))
  (Rendering|Material|SetVectorParameterValue (Variables|Default|GetDecalMaterialInstance) "CustomColor" _returnvalue :!class /Script/Engine.MaterialInstanceDynamic)
  (Effects|Components|ParticleSystem|SetVectorParameter _ns_gravityeffect "BoxSize" (* (Variables|Default|GetBoxExtend) 2.0))
  (Niagara|SetNiagaraVariable(Float) _ns_gravityeffect "SpawnRate" (Variables|Default|GetSpawnRate))
  (Effects|Components|ParticleSystem|SetVectorParameter _ns_gravityeffect "GravityDirection" _direction)
  (Niagara|SetNiagaraVariable(LinearColor) _ns_gravityeffect "GravityColor" _returnvalue))