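; BP_GravityEffect is a box-shaped Niagara effect that visualizes the current gravity direction and color.
; The construction script sizes the box and effect, sets spawn rate and starts the direction at +Z.
; On gravity changes, it waits briefly, then passes the new direction and MPC_World's CurrentGravityColor to Niagara.
; GetGravityColor, not called here, blends per-axis MPC colors by SelectAxe.
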(event Custom|Evt_OnGravityChange
  (params (Data :type S%20Gravity%20Data%20Structure))
  (bind _ns_gravityeffect (Variables|Default|GetNS_GravityEffect))
  (Utilities|FlowControl|Delay 0.2)
  (Effects|Components|ParticleSystem|SetVectorParameter _ns_gravityeffect "GravityDirection" (.Direction (Utilities|Struct|BreakS_GravityData Data)))
  (bind _returnvalue (Rendering|Material|GetVectorParameterValue "/Game/04_Material/Level/ParameterCollection/MPC_World.MPC_World" "CurrentGravityColor" :!class /Script/Engine.KismetMaterialLibrary))
  (Niagara|SetNiagaraVariable(LinearColor) _ns_gravityeffect "GravityColor" _returnvalue))

(event EventBeginPlay
  (EventDispatchers|BindEventtoOnGravityChange (CallFunction|GetGSGravity) (delegate Custom|Evt_OnGravityChange)))

(event EventTick
  (params (DeltaSeconds :type Float%20%28single-precision%29)))

(fn ConstructionScript
  (bind _ns_gravityeffect (Variables|Default|GetNS_GravityEffect))
  (Components|Box|SetBoxExtent (Variables|Default|GetAreaEffect) (Variables|Default|GetBoxExtend) true)
  (Effects|Components|ParticleSystem|SetVectorParameter _ns_gravityeffect "BoxSize" (* (Variables|Default|GetBoxExtend) 2.0))
  (Niagara|SetNiagaraVariable(Float) _ns_gravityeffect "SpawnRate" (Variables|Default|GetSpawnRate))
  (Effects|Components|ParticleSystem|SetVectorParameter _ns_gravityeffect "GravityDirection" "0, 0,1.000000"))

(fn GetGravityColor
  (bind _returnvalue (Rendering|Material|GetVectorParameterValue "/Game/04_Material/Level/ParameterCollection/MPC_World.MPC_World" "SelectAxe" :!class /Script/Engine.KismetMaterialLibrary))
  (bind _returnvalue_2 (Rendering|Material|GetVectorParameterValue "/Game/04_Material/Level/ParameterCollection/MPC_World.MPC_World" "X-" :!class /Script/Engine.KismetMaterialLibrary))
  (bind _returnvalue_3 (Rendering|Material|GetVectorParameterValue "/Game/04_Material/Level/ParameterCollection/MPC_World.MPC_World" "X+" :!class /Script/Engine.KismetMaterialLibrary))
  (bind _returnvalue_4 (Rendering|Material|GetVectorParameterValue "/Game/04_Material/Level/ParameterCollection/MPC_World.MPC_World" "Y-" :!class /Script/Engine.KismetMaterialLibrary))
  (bind _returnvalue_5 (Rendering|Material|GetVectorParameterValue "/Game/04_Material/Level/ParameterCollection/MPC_World.MPC_World" "Y+" :!class /Script/Engine.KismetMaterialLibrary))
  (bind _returnvalue_6 (Rendering|Material|GetVectorParameterValue "/Game/04_Material/Level/ParameterCollection/MPC_World.MPC_World" "Z-" :!class /Script/Engine.KismetMaterialLibrary))
  (bind _returnvalue_7 (Rendering|Material|GetVectorParameterValue "/Game/04_Material/Level/ParameterCollection/MPC_World.MPC_World" "Z+" :!class /Script/Engine.KismetMaterialLibrary))
  (return (Math|Color|Lerp(LinearColor) (Math|Color|Lerp(LinearColor) (Math|Color|Lerp(LinearColor) _returnvalue_6 _returnvalue_7 (/ (+ (.B (Math|Color|BreakColor _returnvalue)) 1.0) 2.0)) (Math|Color|Lerp(LinearColor) _returnvalue_4 _returnvalue_5 (/ (+ (.G (Math|Color|BreakColor _returnvalue)) 1.0) 2.0)) (Math|Float|Absolute(Float) (.G (Math|Color|BreakColor _returnvalue)))) (Math|Color|Lerp(LinearColor) _returnvalue_2 _returnvalue_3 (/ (+ (.R (Math|Color|BreakColor _returnvalue)) 1.0) 2.0)) (Math|Float|Absolute(Float) (.R (Math|Color|BreakColor _returnvalue))))))