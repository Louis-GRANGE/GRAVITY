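; BP_SetDefaultWorldGravity is a placed actor that registers a world gravity entry on BeginPlay.
; It pushes the reversed Arrow forward vector and the Arrow location onto the GS gravity stack, with itself as sender.
; The construction script tints the Arrow by gravity direction and resets its scale.
; When overlap with OusideAutoKillArea ends, it sends OnActorGoOutsideMessage to the area, its owner and the exiting actor.
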(event OnComponentEndOverlap(OusideAutoKillArea)
  (params (OverlappedComponent :type Primitive%20Component%20Object%20Reference) (OtherActor :type Actor%20Object%20Reference) (OtherComp :type Primitive%20Component%20Object%20Reference) (OtherBodyIndex :type Integer))
  (Class|BPIKillArea|OnActorGoOutside(Message) OverlappedComponent)
  (Class|BPIKillArea|OnActorGoOutside(Message) (Components|GetOwner OverlappedComponent))
  (Class|BPIKillArea|OnActorGoOutside(Message) OtherActor))

(event EventBeginPlay
  (bind _arrow (Variables|Default|GetArrow))
  (Default|AddGravityStack (CallFunction|GetGSGravity) (Utilities|Struct|MakeS_GravityData (Variables|Default|GetApply%20To) (* (Math|Vector|GetForwardVector _arrow) -1.0) -9.8 (Transformation|GetWorldLocation _arrow) -1.0 self)))

(event Collision|EventActorBeginOverlap
  (params (OtherActor :type Actor%20Object%20Reference)))

(event EventTick
  (params (DeltaSeconds :type Float%20%28single-precision%29)))

(fn ConstructionScript
  (bind _returnvalue (CallFunction|GetGravityColor (* (Math|Vector|GetForwardVector (Variables|Default|GetArrow)) -1.0)))
  (Variables|/Script/Engine.ArrowComponent|SetArrowColor (Variables|Default|GetArrow) (Math|Conversions|ToColor(LinearColor) _returnvalue))
  (Transformation|SetWorldScale3D (Variables|Default|GetArrow) "1.000000,1.000000,1.000000"))