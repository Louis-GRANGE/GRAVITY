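; Main menu camera Blueprint that keeps itself aimed at the middle of the scene's BP_GravityActorComponent actors.
; On BeginPlay it gathers and caches all actors of that class.
; Each Tick, CalculateCentroid averages their current locations, and the actor rotates via FindLookAtRotation to face that point without changing its own position.
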(event EventBeginPlay
  (bind _outactors (Actor|GetAllActorsOfClass "/Game/05_BP/Objects/GravityObject/BP_GravityActor-Component.BP_GravityActor-Component_C"))
  (Variables|Default|SetOut%20Actors _outactors))

(event Collision|EventActorBeginOverlap
  (params (OtherActor :type Actor%20Object%20Reference)))

(event EventTick
  (params (DeltaSeconds :type Float%20%28single-precision%29))
  (bind _returnvalue (CallFunction|CalculateCentroid (Variables|Default|GetOut%20Actors)))
  (Transformation|SetActorRotation (Math|Rotator|FindLookatRotation (Transformation|GetActorLocation) _returnvalue)))

(fn ConstructionScript
  (|CallParentFunction))

(fn CalculateCentroid
  (params (Actors :type Array%20of%20Actor%20Object%20References))
  (for _array_element Actors
    (LocalVariables|SetCentroid (+ (Transformation|GetActorLocation _array_element) (LocalVariables|GetCentroid))))
  (return (/ (LocalVariables|GetCentroid) (Utilities|Array|Length Actors))))