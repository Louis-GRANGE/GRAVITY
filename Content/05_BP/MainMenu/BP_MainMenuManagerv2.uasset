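; BP_MainMenuManagerv2 is a main menu manager that periodically changes the gravity direction while the menu runs.
; On BeginPlay it caches the BP_MainCamera actor and starts a fast looping timer.
; Every random few seconds, UpdateMainMenu passes a random axis-aligned direction to GetGSGravity's UpdateGravityTo.
; The level streaming and level instance nodes are unconnected and never run.
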(event Custom|UpdateMainMenu
  (if (> (Utilities|Time|GetTimeSeconds) (Variables|Default|GetTime))
    (Default|UpdateGravityto (CallFunction|GetGSGravity) "NewEnumerator0" (Utilities|Select :Index (Math|Random|RandomIntegerinRange 0 5) :Option%200 "1.000000,0.000000,0.000000" :Option%201 "-1.000000,0.000000,0.000000" :Option%202 "0.000000,1.000000,0.000000" :Option%203 "0.000000,-1.000000, 0" :Option%204 "0, 0,1.000000" :Option%205 "0.000000,0.000000,-1.000000") -9.8 "0, 0, 0")
    (Variables|Default|SetTime (+ (Utilities|Time|GetTimeSeconds) (Math|Random|RandomFloatinRange 2.0 1e+01)))))

(event EventBeginPlay
  (Variables|Default|SetTime (Math|Random|RandomFloatinRange 2.0 1e+01))
  (Utilities|Time|SetTimerbyEvent (EventDispatchers|CreateEvent :!event Custom|UpdateMainMenu) 0.1 true)
  (bind _returnvalue (Actor|GetActorOfClass "/Game/05_BP/MainMenu/BP_MainCamera.BP_MainCamera_C"))
  (Variables|Default|SetCurrentCamera _returnvalue))

(event Collision|EventActorBeginOverlap
  (params (OtherActor :type Actor%20Object%20Reference)))

(event EventTick
  (params (DeltaSeconds :type Float%20%28single-precision%29)))

(fn ConstructionScript)